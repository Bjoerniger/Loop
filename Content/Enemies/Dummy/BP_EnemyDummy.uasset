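; Dummy enemy for a side-scroller that takes damage from player bullets, shows a health bar and breaks on death.
; Box overlaps detect bullets by object name and the player's TriggerCheck component, disabling enemy collision during dashes until a timer restores the box.
; Tick updates the health ratio and, at zero health, swaps the static mesh for a physics-simulated destructible.
; The HealthUI widget receives a reference to the enemy.
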(event `self.ReceiveBeginPlay`
  (`|ExecutionSequence`
    (:`then_0`
      (set `self.healthActual` (`self.healthMax`))
      (bind _returnvalue (`|CreateWidget` "/Game/UI/UI_EnemyHealthBPBar.UI_EnemyHealthBPBar_C"))
      (set `self.Ref_HealthWidget` _returnvalue))
    (:`then_1`
      (bind _asui_enemy_health_bpbar (cast `/Game/UI/UI_EnemyHealthBPBar` (`WidgetComponent.GetUserWidgetObject` (`self.HealthUI`))))
      (set `/Game/UI/UI_EnemyHealthBPBar.Enemy` self _asui_enemy_health_bpbar))))

(event `self.Box.OnComponentBeginOverlap`
  (params (OverlappedComponent :type "PrimitiveComponent Object Reference") (OtherActor :type "Actor Object Reference") (OtherComp :type "PrimitiveComponent Object Reference") (OtherBodyIndex :type Integer) (bFromSweep :type Boolean) (SweepResult :type "HitResult Structure (by ref)"))
  (bind _box (`self.Box`))
  ;[1 1 1] hit by player and death
  (if (`KismetStringLibrary.Contains` (`KismetSystemLibrary.GetObjectName` OtherActor) "PlayerBullet")
    (set `self.healthActual` (- (`self.healthActual`) (`self.dmgCast`)))
    (else
      ;[1 1 1] dash
      (if (`ActorComponent.ComponentHasTag` OtherComp "TriggerCheck")
        (bind _asside_scroller_character (cast `/Game/SideScrollerCPP/Blueprints/SideScrollerCharacter` (`GameplayStatics.GetPlayerCharacter` 0)))
        (set `self.beenDashed` true)
        (if (`self.isAlive`)
          (if (`UnholyCharacter.isDashing` _asside_scroller_character)
            (`PrimitiveComponent.SetCollisionProfileName` _box "NoEnemyCollision" :!label _label)
            (`PrimitiveComponent.SetCollisionProfileName` (`self.EnemyModel_Static`) "NoEnemyCollision")
            (elif (<= (`self.healthActual`) 0.0)
              (goto _label)
              (else
                (`PrimitiveComponent.SetCollisionProfileName` _box "EnemyCollision")
                (`PrimitiveComponent.SetCollisionProfileName` (`self.EnemyModel_Static`) "EnemyCollision"))))
          (else
            (goto _label)))))))

(event `self.ReceiveTick`
  (params (DeltaSeconds :type "Float (single-precision)"))
  (bind _enemymodel_destructable (`self.EnemyModel_Destructable`))
  (bind _enemymodel_static (`self.EnemyModel_Static`))
  (`|ExecutionSequence`
    (:`then_0`
      (if (<= (`self.HealthActual`) 0.0)
        (set `self.isAlive` false)))
    (:`then_1`
      ;[1 1 1] set health %
      (set `self.HealthReturnValue` (/ (`self.HealthActual`) (`self.HealthMax`))))
    (:`then_2`
      ;[1 1 1] dash
      (if (`self.beenDashed`)
        (if (< (`self.dashedTimer`) (`self.dashedTimerMax`))
          (set `self.dashedTimer` (+ DeltaSeconds (`self.dashedTimer`)))
          (else
            (set `self.beenDashed` false)
            (set `self.dashedTimer` 0.0)
            (`PrimitiveComponent.SetCollisionProfileName` (`self.Box`) "EnemyCollision")))))
    (:`then_3`
      ;[1 1 1] on death
      (if (not (`self.isAlive`))
        (`SceneComponent.SetHiddenInGame` _enemymodel_static true false)
        (`SceneComponent.SetVisibility` _enemymodel_static false false)
        (`PrimitiveComponent.SetCollisionEnabled` _enemymodel_static "NoCollision")
        (`SceneComponent.SetHiddenInGame` _enemymodel_destructable false false)
        (`PrimitiveComponent.SetEnableGravity` _enemymodel_destructable true)
        (`PrimitiveComponent.WakeRigidBody` _enemymodel_destructable "None")
        (`PrimitiveComponent.SetSimulatePhysics` _enemymodel_destructable true)
        (`PrimitiveComponent.SetCollisionEnabled` _enemymodel_destructable "QueryAndPhysics")))
    (:`then_4`
      (set `self.gotGrav` (`PrimitiveComponent.IsGravityEnabled` (`self.EnemyModel_Destructable`))))))

(fn `UserConstructionScript`)