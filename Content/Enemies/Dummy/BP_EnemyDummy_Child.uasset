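; Child Blueprint of the enemy dummy that toggles a destructible cube piece based on the state of the enemy's destructible model.
; Each Tick polls whether gravity is enabled on EnemyModelDestructable: if so, CubeDM becomes visible and collidable and Cube starts simulating physics.
; Otherwise CubeDM stays hidden without collision.
; An unconnected radius damage call on CubeDM never runs.
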(event `self.ReceiveTick`
  (params (DeltaSeconds :type "Float (single-precision)"))
  (bind _cube_dm (`self.Cube_DM`))
  (`parent.ReceiveTick` DeltaSeconds)
  (if (`PrimitiveComponent.IsGravityEnabled` (`self.EnemyModel_Destructable`))
    (`PrimitiveComponent.SetCollisionEnabled` _cube_dm "QueryAndPhysics")
    (`SceneComponent.SetVisibility` _cube_dm true false)
    (`PrimitiveComponent.SetSimulatePhysics` (`self.Cube`) true)
    (else
      (`PrimitiveComponent.SetCollisionEnabled` _cube_dm "NoCollision")
      (`SceneComponent.SetVisibility` _cube_dm false false))))

(fn `UserConstructionScript`
  (`parent.UserConstructionScript`))