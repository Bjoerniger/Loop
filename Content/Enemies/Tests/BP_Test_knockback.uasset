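; Test enemy character that gets knocked away from player 0 after being kicked.
; Tick polls the BeenKicked flag, prints the player-to-self offset with X zeroed, launches the character along it, then clears the flag.
; The scaled offset is not normalized, so knockback strength grows with distance; XY velocity is overridden while Z is additive.
; Nothing in this graph sets BeenKicked to true.
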(event `self.ReceiveTick`
  (params (DeltaSeconds :type "Float (single-precision)"))
  (bind (_returnvalue_x _returnvalue_y _returnvalue_z) (`KismetMathLibrary.BreakVector` (`self.K2_GetActorLocation` self)))
  (bind (_returnvalue_x_2 _returnvalue_y_2 _returnvalue_z_2) (`KismetMathLibrary.BreakVector` (`SceneComponent.K2_GetComponentLocation` (`Actor.RootComponent` (`GameplayStatics.GetPlayerCharacter` 0)))))
  (bind _returnvalue (- (`KismetMathLibrary.MakeVector` 0.0 _returnvalue_y _returnvalue_z) (`KismetMathLibrary.MakeVector` 0.0 _returnvalue_y_2 _returnvalue_z_2)))
  (if (`self.been kicked`)
    (`KismetSystemLibrary.PrintString` (`KismetStringLibrary.Conv_VectorToString` _returnvalue))
    (`self.LaunchCharacter` (* _returnvalue 5.0) true)
    (set `self.been kicked` false)))

(fn `UserConstructionScript`)