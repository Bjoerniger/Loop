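; Enemy Blueprint for a ball-type enemy with an advanced weapon component, layered on shared Enemy class logic.
; AggroRange overlaps forward to OnOverlapBegin, only while alive, and to OnOverlapEnd on exit.
; Each tick the weapon component copies collision, gravity and physics simulation from the static enemy model and is visible only while health is above zero.
; The AggroSphere overlap event is an empty stub.
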(event `self.aggroSphere.OnComponentBeginOverlap`
  (params (OverlappedComponent :type "PrimitiveComponent Object Reference") (OtherActor :type "Actor Object Reference") (OtherComp :type "PrimitiveComponent Object Reference") (OtherBodyIndex :type Integer) (bFromSweep :type Boolean) (SweepResult :type "HitResult Structure (by ref)"))
  ;[1 1 1] collisions
)

(event `self.aggroRange.OnComponentBeginOverlap`
  (params (OverlappedComponent :type "PrimitiveComponent Object Reference") (OtherActor :type "Actor Object Reference") (OtherComp :type "PrimitiveComponent Object Reference") (OtherBodyIndex :type Integer) (bFromSweep :type Boolean) (SweepResult :type "HitResult Structure (by ref)"))
  ;[1 1 1] collisions
  (bind _asenemy (cast `Enemy` self))
  (if (`Enemy.bIsAlive` _asenemy)
    (`self.OnOverlapBegin` _asenemy OverlappedComponent OtherActor OtherComp OtherBodyIndex bFromSweep SweepResult)))

(event `self.ReceiveTick`
  (params (DeltaSeconds :type "Float (single-precision)"))
  (bind _enemymodel_static (`self.EnemyModel_Static`))
  (bind _enemy_ball_advanced_weapon (`self.Enemy_Ball_Advanced_Weapon`))
  (`parent.ReceiveTick` DeltaSeconds)
  (`|ExecutionSequence`
    (:`then_0`
      (`PrimitiveComponent.SetCollisionEnabled` _enemy_ball_advanced_weapon (`PrimitiveComponent.GetCollisionEnabled` _enemymodel_static))
      (`PrimitiveComponent.SetEnableGravity` _enemy_ball_advanced_weapon (`PrimitiveComponent.IsGravityEnabled` _enemymodel_static))
      (`PrimitiveComponent.SetSimulatePhysics` _enemy_ball_advanced_weapon (`SceneComponent.IsSimulatingPhysics` _enemymodel_static "None"))
      (if (> (`self.healthReturnValue`) 0.0)
        (`SceneComponent.SetVisibility` _enemy_ball_advanced_weapon true false)
        (else
          (`SceneComponent.SetVisibility` _enemy_ball_advanced_weapon false false))))))

(event `self.aggroRange.OnComponentEndOverlap`
  (params (OverlappedComponent :type "PrimitiveComponent Object Reference") (OtherActor :type "Actor Object Reference") (OtherComp :type "PrimitiveComponent Object Reference") (OtherBodyIndex :type Integer))
  ;[1 1 1] collisions
  (`self.OnOverlapEnd` OverlappedComponent OtherActor OtherComp OtherBodyIndex))

(fn `UserConstructionScript`
  (`parent.UserConstructionScript`))