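; Base enemy Blueprint for a side-scroller, handling health, damage, death and target display, with its X position locked.
; Tick polls hit and crit flags, identifying bullets and stomps by object-name substring to apply damage.
; Player contact starts a timer, and dashing switches the body trigger's collision off until it expires.
; Death clears the player's homing target and swaps the static model for a physics-simulated destructible.
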(event `self.ReceiveBeginPlay`
  (bind _returnvalue_x (`KismetMathLibrary.BreakVector` (`self.K2_GetActorLocation`)))
  (`|ExecutionSequence`
    (:`then_0`
      (set `self.x location fix` _returnvalue_x))
    (:`then_1`
      ;[1 1 1] widgets
      (bind _returnvalue (`|CreateWidget` "/Game/UI/Enemy/UI_Enemy_AggroTimer.UI_Enemy_AggroTimer_C"))
      (set `self.Ref_HealthWidget` _returnvalue))
    (:`then_2`
      (bind _returnvalue_2 (`|CreateWidget` "/Game/UI/Enemy/UI_Enemy_AggroTimer.UI_Enemy_AggroTimer_C"))
      (set `self.Ref_AggroWidget` _returnvalue_2))
    (:`then_3`
      (bind _returnvalue_3 (`|CreateWidget` "/Game/UI/Enemy/UI_Enemy_IsTargeted.UI_Enemy_IsTargeted_C"))
      (set `self.Ref_TargetWidget` _returnvalue_3))
    (:`then_4`
      (bind _outactors (`GameplayStatics.GetAllActorsOfClass` "/Game/Objects/BP_HorizonCube.BP_HorizonCube_C"))
      (for _array_element _outactors
        (set `self.horizonCube` _array_element)))))

(event `self.ReceiveTick`
  (params (DeltaSeconds :type "Float (single-precision)"))
  (bind _core (`self.Core`))
  (bind _bodytriggervolume (`self.BodyTriggerVolume`))
  (bind _enemymodel_static (`self.EnemyModel_static`))
  (bind _enemymodel_destructable (`self.EnemyModel_Destructable`))
  (bind _x_location_fix (`self.x location fix`))
  (bind _thehitcomp (`self.theHitComp`))
  (bind _enemymodel_destructable_2 (`self.EnemyModel_Destructable`))
  (bind _returnvalue (`KismetSystemLibrary.GetObjectName` (`self.theHitMan`)))
  (bind _returnvalue_2 (`KismetSystemLibrary.GetObjectName` (`self.theHitMan`)))
  (bind (_returnvalue_x _returnvalue_y _returnvalue_z) (`KismetMathLibrary.BreakVector` (`self.K2_GetActorLocation` self)))
  (bind (_relativerotation_roll _relativerotation_pitch _relativerotation_yaw) (`KismetMathLibrary.BreakRotator` (`SceneComponent.RelativeRotation` _core)))
  (`|ExecutionSequence`
    (:`then_0`
      ;[1 1 1] vars
      ;;[1 1 1] death
      (if (<= (`self.healthValue`) 0.0)
        (set `self.bIsAlive` false)))
    (:`then_1`
      ;;[1 1 1] set health %
      (set `self.healthReturnValue` (/ (`self.healthValue`) (`self.healthMax`))))
    (:`then_2`
      ;[1 1 1] dash
      (if (`self.bBeenDashed`)
        (if (`self.bIsAlive`)
          (if (< (`self.dashedTimerValue`) (`self.dashedTimerMax`))
            (set `self.dashedTimerValue` (+ DeltaSeconds (`self.dashedTimerValue`)))
            (else
              (set `self.bBeenDashed` false)
              (set `self.dashedTimerValue` 0.0)
              (`/Engine/EditorBlueprintResources/StandardMacros.IsValid` _bodytriggervolume
                (:`Is Valid`
                  (`PrimitiveComponent.SetCollisionProfileName` _bodytriggervolume "EnemyCollision"))))))))
    (:`then_3`
      ;[1 1 1] on death
      (if (not (`self.bIsAlive`))
        ;;[1 1 1] reset homing target on player
        (bind _asunholy_character (cast `UnholyCharacter` (`GameplayStatics.GetPlayerCharacter` 0)))
        (if (== (`UnholyCharacter.homingTarget` _asunholy_character) self)
          (set `UnholyCharacter.homingTarget` null _asunholy_character))
        (`/Engine/EditorBlueprintResources/StandardMacros.DoOnce` false
          (:`Completed`
            (`GameplayStatics.PlaySoundAtLocation` "/Game/Sounds/cues/SND_Enemy_Death.SND_Enemy_Death" (`self.K2_GetActorLocation`) (struct) 1.0 1.0 0.0 null null null)
            (`PrimitiveComponent.SetCollisionEnabled` (`self.CapsuleComponent`) "NoCollision")
            (`PrimitiveComponent.SetCollisionProfileName` (`self.Core`) "NoEnemyCollision")
            (`SceneComponent.SetVisibility` _enemymodel_static false false)
            (`SceneComponent.SetHiddenInGame` _enemymodel_static true false)
            (`SceneComponent.SetHiddenInGame` _enemymodel_destructable false false)
            (`PrimitiveComponent.SetEnableGravity` _enemymodel_destructable true)
            (`PrimitiveComponent.WakeRigidBody` _enemymodel_destructable "None")
            (`PrimitiveComponent.SetSimulatePhysics` _enemymodel_destructable true)
            (`/Engine/EditorBlueprintResources/StandardMacros.IsValid` _enemymodel_destructable
              (:`Is Valid`
                (`PrimitiveComponent.SetCollisionEnabled` _enemymodel_destructable "QueryAndPhysics")))))))
    (:`then_4`
      (set `self.bGotGrav` (`PrimitiveComponent.IsGravityEnabled` (`self.EnemyModel_Destructable`))))
    (:`then_5`
      ;[1 1 1] hit by player
      (if (`self.bBeenHit`)
        (if (`KismetStringLibrary.Contains` _returnvalue_2 "PlayerBullet")
          (set `self.healthValue` (- (`self.healthValue`) (`self.damageCast`)) :!label _label)
          (set `self.bBeenHit` false)
          (elif (`KismetStringLibrary.Contains` _returnvalue_2 "Stomper")
            (goto _label)
            (elif (`KismetSystemLibrary.IsValid` _thehitcomp)
              (if (`ActorComponent.ComponentHasTag` _thehitcomp "TriggerCheck")
                (bind _asside_scroller_character (cast `/Game/SideScrollerCPP/Blueprints/SideScrollerCharacter` (`GameplayStatics.GetPlayerCharacter` 0)))
                (set `self.bBeenDashed` true)
                (if (`self.bIsAlive`)
                  (if (`UnholyCharacter.isDashing` _asside_scroller_character)
                    (`PrimitiveComponent.SetCollisionProfileName` _bodytriggervolume "NoEnemyCollision" :!label _label_2)
                    (elif (<= (`self.healthValue`) 0.0)
                      (goto _label_2)
                      (else
                        (`/Engine/EditorBlueprintResources/StandardMacros.IsValid` _bodytriggervolume
                          (:`Is Valid`
                            (`PrimitiveComponent.SetCollisionProfileName` _bodytriggervolume "EnemyCollision"))))))
                  (else
                    (goto _label_2)))))))))
    (:`then_6`
      ;[1 1 1] collision settings
      (if (`self.bGotGrav`)
        (if (`PrimitiveComponent.IsGravityEnabled` (`self.EnemyModel_Destructable`))
          (`PrimitiveComponent.SetCollisionEnabled` _enemymodel_destructable_2 "QueryAndPhysics")
          (`SceneComponent.SetVisibility` _enemymodel_destructable_2 true false)
          (`PrimitiveComponent.SetSimulatePhysics` (`self.Core`) true)
          (else
            (`PrimitiveComponent.SetCollisionEnabled` _enemymodel_destructable_2 "NoCollision")
            (`SceneComponent.SetVisibility` _enemymodel_destructable_2 false false)))))
    (:`then_7`
      ;[1 1 1] simple core rotation
      (if (`self.bIsAlive`)
        (`SceneComponent.K2_AddLocalRotation` _core (`KismetMathLibrary.MakeRotator` (+ _relativerotation_roll -1.0) (+ _relativerotation_pitch 1.0) (+ _relativerotation_yaw 2.0)) false false)))
    (:`then_9`
      ;[1 1 1] crit by player
      (if (`self.bCanReceiveCriticalHit`)
        (if (`self.bBeenCrit`)
          (if (`KismetStringLibrary.Contains` _returnvalue "PlayerBullet")
            (bind _asunholy_character_2 (cast `UnholyCharacter` (`GameplayStatics.GetPlayerCharacter` 0)))
            (set `self.healthValue` (- (`self.healthValue`) (* (`self.damageCast`) (`UnholyCharacter.critMultiplier` _asunholy_character_2))))
            (set `self.bBeenCrit` false)
            (elif (`KismetStringLibrary.Contains` _returnvalue "Stomper")
              (set `self.healthValue` (- (`self.healthValue`) (`self.damageCast`)))
              (set `self.bBeenCrit` false))))))
    (:`then_10`
      ;[0.8714 1 0.4735] lock axis
      (if (!= _returnvalue_x _x_location_fix)
        (`self.K2_SetActorLocation` (`KismetMathLibrary.MakeVector` (`KismetMathLibrary.Conv_IntToDouble` (`KismetMathLibrary.FCeil` _x_location_fix)) _returnvalue_y _returnvalue_z))))
    (:`then_11`
      ;[1 1 1] target square stuff
      (bind _asui_enemy_is_targeted (cast `/Game/UI/Enemy/UI_Enemy_IsTargeted` (`WidgetComponent.GetUserWidgetObject` (`self.UI_Target`))))
      (set `/Game/UI/Enemy/UI_Enemy_IsTargeted.OwnerIsAlive` (`self.bIsAlive`) _asui_enemy_is_targeted)
      (set `/Game/UI/Enemy/UI_Enemy_IsTargeted.OwnerIsTarget` (`self.bIsHomingTarget`) _asui_enemy_is_targeted))))

(fn `UserConstructionScript`)