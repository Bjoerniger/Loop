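; Ball enemy Blueprint that presents combat state for several attack types: shooter, alerter, charger, defender and mines.
; An aggro sphere forwards player-range overlaps to inherited or shared handlers.
; Tick polls state to update materials, health/shield and aggro-timer widgets, crit effect, death hiding, and an aim laser scaled by player distance.
; Tick also triggers the one-shot charger explosion and caches patrol waypoints; kick launch code is disconnected.
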(event `self.ReceiveBeginPlay`
  (bind (_relativescale3d_x _relativescale3d_y _relativescale3d_z) (`KismetMathLibrary.BreakVector` (`SceneComponent.RelativeScale3D` (`self.BP_EnemyAimLaser`))))
  (`parent.ReceiveBeginPlay`)
  (`|ExecutionSequence`
    (:`then_0`
      ;[1 1 1] laser length stuff
      ;;[1 1 1] set laser initial length
      (set `self.baselaserLength` _relativescale3d_z))
    (:`then_1`
      (`SphereComponent.SetSphereRadius` (`self.aggroRangeDisplay`) (`self.aggroRange`) true))))

(event `self.aggroSphere.OnComponentBeginOverlap`
  (params (OverlappedComponent :type "PrimitiveComponent Object Reference") (OtherActor :type "Actor Object Reference") (OtherComp :type "PrimitiveComponent Object Reference") (OtherBodyIndex :type Integer) (bFromSweep :type Boolean) (SweepResult :type "HitResult Structure (by ref)"))
  ;[1 1 1] collisions
)

(event `self.aggroRangeDisplay.OnComponentBeginOverlap`
  (params (OverlappedComponent :type "PrimitiveComponent Object Reference") (OtherActor :type "Actor Object Reference") (OtherComp :type "PrimitiveComponent Object Reference") (OtherBodyIndex :type Integer) (bFromSweep :type Boolean) (SweepResult :type "HitResult Structure (by ref)"))
  ;[1 1 1] collisions
  (if (`self.bIsAlive`)
    (`self.OnOverlapBegin` OverlappedComponent OtherActor OtherComp OtherBodyIndex bFromSweep SweepResult)))

(event `self.ReceiveTick`
  (params (DeltaSeconds :type "Float (single-precision)"))
  (bind _returnvalue (`self.K2_GetActorLocation`))
  (bind _ui_health (`self.UI_Health`))
  (bind _bp_enemyaimlaser (`self.BP_EnemyAimLaser`))
  (bind _aggrorangedisplay (`self.aggroRangeDisplay`))
  (bind _enemymodel_static (`self.EnemyModel_Static`))
  (bind _aggrodisplaysphere (`self.AggroDisplaySphere`))
  (bind _enemymodel_weapon (`self.enemyModel_weapon`))
  (bind _defendershieldhealthvalue (`self.defenderShieldHealthValue`))
  (bind _patrolwaypoints (`self.patrolWayPoints`))
  (bind _enemymodel_static_2 (`self.EnemyModel_Static`))
  (bind _aggrostate (`self.aggroState`))
  (bind _core (`self.Core`))
  (bind _returnvalue_2 (`SceneComponent.GetRelativeTransform` _bp_enemyaimlaser))
  (bind _returnvalue_3 (- (`self.aggroInitTimerMax`) (`self.aggroInitTimerValue`)))
  (bind _returnvalue_4 (* (/ (`self.aggroRange`) 600.0) 12.0))
  (`parent.ReceiveTick` DeltaSeconds)
  (`|ExecutionSequence`
    (:`then_0`
      ;[1 1 1] on death
      (`PrimitiveComponent.SetCollisionEnabled` _enemymodel_static (`PrimitiveComponent.GetCollisionEnabled` _enemymodel_static))
      (`PrimitiveComponent.SetEnableGravity` _enemymodel_static (`PrimitiveComponent.IsGravityEnabled` _enemymodel_static))
      (`PrimitiveComponent.SetSimulatePhysics` _enemymodel_static (`SceneComponent.IsSimulatingPhysics` _enemymodel_static "None"))
      (if (> (`self.healthReturnValue`) 0.0)
        (`SceneComponent.SetVisibility` _enemymodel_static true false)
        (`SceneComponent.SetVisibility` (`self.enemyModel_weapon`) true false)
        (else
          (set `self.bIsAlive` false)
          (`SceneComponent.SetVisibility` _enemymodel_static false true)
          (`SceneComponent.SetVisibility` (`self.enemyModel_weapon`) false true)
          (`SceneComponent.SetVisibility` (`self.BP_EnemyAimLaser`) false true)
          (`PrimitiveComponent.SetCollisionEnabled` _enemymodel_static "NoCollision")
          (`PrimitiveComponent.SetCollisionEnabled` (`self.enemyModel_weapon`) "NoCollision")
          (`SceneComponent.SetHiddenInGame` (`self.BP_EnemyAimLaser`) true true))))
    (:`then_1`
      ;[1 1 1] aggro mat
      (if (`|EnumEquality` _aggrostate "EAS_neutral")
        (`PrimitiveComponent.SetMaterial` _enemymodel_static_2 2 "/Game/Materials/MAT_enemyAggro_neutral.MAT_enemyAggro_neutral")
        (`PrimitiveComponent.SetMaterial` _core 0 "/Game/Materials/MAT_enemyAggro_neutral.MAT_enemyAggro_neutral")
        (elif (`|EnumEquality` _aggrostate "EAS_allert")
          (`PrimitiveComponent.SetMaterial` _enemymodel_static_2 2 "/Game/Materials/MAT_enemyAggro_allerted.MAT_enemyAggro_allerted")
          (`PrimitiveComponent.SetMaterial` _core 0 "/Game/Materials/MAT_enemyAggro_allerted.MAT_enemyAggro_allerted")
          (elif (`|EnumEquality` _aggrostate "EAS_attack")
            (`PrimitiveComponent.SetMaterial` _enemymodel_static_2 2 "/Game/Materials/MAT_enemyAggro_attacking.MAT_enemyAggro_attacking")
            (`PrimitiveComponent.SetMaterial` _core 0 "/Game/Materials/MAT_enemyAggro_attacking.MAT_enemyAggro_attacking")
            (elif (`|EnumEquality` _aggrostate "EAS_defense")
              (`PrimitiveComponent.SetMaterial` _enemymodel_static_2 2 "/Game/Materials/MAT_enemyAggro_defending.MAT_enemyAggro_defending")
              (`PrimitiveComponent.SetMaterial` _core 0 "/Game/Materials/MAT_enemyAggro_defending.MAT_enemyAggro_defending"))))))
    (:`then_2`
      ;[1 1 1] kick mechanic
      (if (`self.bIsKickable`)
        _))
    (:`then_3`
      ;[1 1 1] laser length stuff
      ;;[1 1 1] set laser visibility
      (if (`self.bIsAlive`)
        (if (`self.bPlayerIsInAggroRange`)
          (`SceneComponent.SetVisibility` _bp_enemyaimlaser (`self.bCanSeePlayer`) false)
          (else
            (`SceneComponent.SetVisibility` _bp_enemyaimlaser false true :!label _label)))
        (else
          (goto _label))))
    (:`then_4`
      ;;[1 1 1] set laser adaptive range to player
      (`SceneComponent.SetRelativeScale3D` _bp_enemyaimlaser (`KismetMathLibrary.MakeVector` (.x (.scale _returnvalue_2)) (.y (.scale _returnvalue_2)) (* (/ (`self.GetDistanceTo` (`GameplayStatics.GetPlayerCharacter` 0)) (`SphereComponent.SphereRadius` (`self.aggroRangeDisplay`))) (`self.baselaserLength`)))))
    (:`then_5`
      ;[1 1 1] health bar widget && aggro
      (bind _asui_enemy_health (cast `/Game/UI/Enemy/UI_Enemy_Health` (`WidgetComponent.GetUserWidgetObject` _ui_health)))
      (`ProgressBar.SetPercent` (`/Game/UI/Enemy/UI_Enemy_Health.healthBar` _asui_enemy_health) (/ (`self.healthValue`) (`self.healthMax`)))
      (if (> _defendershieldhealthvalue 0.0)
        (bind _shieldbar (`/Game/UI/Enemy/UI_Enemy_Health.shieldBar` _asui_enemy_health))
        (`ProgressBar.SetPercent` _shieldbar (/ _defendershieldhealthvalue (`self.defenderShieldHealthMax`)))
        (else
          (`Widget.SetVisibility` _shieldbar "Hidden"))))
    (:`then_6`
      ;[1 1 1] critical hit fx
      (if (`self.bIsAlive`)
        (if (`self.bDisplayCritEffect`)
          (if (< (`self.critDisplayTimerValue`) (`self.critDisplayTimer`))
            (`SceneComponent.SetVisibility` (`self.CritHitDisplay`) true false)
            (set `self.critDisplayTimerValue` (+ (`self.critDisplayTimerValue`) (`GameplayStatics.GetWorldDeltaSeconds`)))
            (else
              (`SceneComponent.SetVisibility` (`self.CritHitDisplay`) false false :!label _label_2)
              (set `self.critDisplayTimerValue` 0.0)
              (set `self.bDisplayCritEffect` false)))
          (else
            (goto _label_2)))
        (else
          (goto _label_2))))
    (:`then_7`
      (`|ExecutionSequence`
        (:`then_0`
          (if (not (> (`self.healthValue`) 0.0))
            (`SceneComponent.SetVisibility` _ui_health false false)
            (`SceneComponent.SetVisibility` (`self.UI_Aggro`) false false)))
        (:`then_1`
          (bind _asui_enemy_aggro_timer (cast `/Game/UI/Enemy/UI_Enemy_AggroTimer` (`WidgetComponent.GetUserWidgetObject` (`self.UI_Aggro`))))
          (if (> _returnvalue_3 0.0)
            (`TextBlock.SetText` (`/Game/UI/Enemy/UI_Enemy_AggroTimer.AggroTimer` _asui_enemy_aggro_timer) (`KismetTextLibrary.Conv_StringToText` (`KismetStringLibrary.GetSubstring` (`KismetStringLibrary.Conv_DoubleToString` _returnvalue_3) 0 3)))
            (else
              (`TextBlock.SetText` (`/Game/UI/Enemy/UI_Enemy_AggroTimer.AggroTimer` _asui_enemy_aggro_timer) "!"))))))
    (:`then_8`
      (if (== (`SphereComponent.SphereRadius` _aggrorangedisplay) 0.0)
        (`SphereComponent.SetSphereRadius` _aggrorangedisplay (`self.aggroRange`) true)))
    (:`then_9`
      ;[1 1 1] set aggro display colour
      (if (`self.bIsAlive`)
        (if (`self.bCanSeePlayer`)
          (if (`self.bPlayerIsInAggroRange`)
            (if (`|EnumEquality` (`self.attackType`) "EAT_allert")
              ;;[1 1 1] allerting
              (`PrimitiveComponent.SetMaterial` _aggrodisplaysphere 0 "/Game/Materials/MAT_Enemy_Allert_Pulse.MAT_Enemy_Allert_Pulse")
              (else
                ;;[1 1 1] has aggro
                (`PrimitiveComponent.SetMaterial` _aggrodisplaysphere 0 "/Game/Materials/MAT_I_Enemy_AggroDisplay.MAT_I_Enemy_AggroDisplay" :!label _label_3)
                (`MeshComponent.SetVectorParameterValueOnMaterials` _aggrodisplaysphere "Emissive Color" (1.0 0.0 0.0))))
            (else
              (if (`|EnumEquality` (`self.aggroState`) "EAS_attack") :!label _label_4
                (goto _label_3)
                (else
                  ;;[1 1 1] no aggro
                  (`PrimitiveComponent.SetMaterial` _aggrodisplaysphere 0 "/Game/Materials/MAT_I_Enemy_AggroDisplay.MAT_I_Enemy_AggroDisplay")
                  (`MeshComponent.SetVectorParameterValueOnMaterials` _aggrodisplaysphere "Emissive Color" (1.0 1.0 1.0))))))
          (else
            (goto _label_4)))
        (else
          ;;[1 1 1] dead
          (`PrimitiveComponent.SetMaterial` _aggrodisplaysphere 0 "/Game/Materials/MAT_I_Enemy_AggroDisplay.MAT_I_Enemy_AggroDisplay")
          (`SceneComponent.SetVisibility` _aggrodisplaysphere false false))))
    (:`then_10`
      ;[1 1 1] set class skin
      (if (`|EnumEquality` (`self.attackType`) "EAT_range")
        (`PrimitiveComponent.SetMaterial` _enemymodel_weapon 0 "/Game/Materials/MAT_Enemy_Main_Shooter.MAT_Enemy_Main_Shooter")
        (elif (`|EnumEquality` (`self.attackType`) "EAT_allert")
          (`PrimitiveComponent.SetMaterial` _enemymodel_weapon 0 "/Game/Materials/MAT_Enemy_Main_Allerter.MAT_Enemy_Main_Allerter")
          (elif (`|EnumEquality` (`self.attackType`) "EAT_range")
            (`PrimitiveComponent.SetMaterial` _enemymodel_weapon 0 "/Game/Materials/MAT_Enemy_Main_Charger.MAT_Enemy_Main_Charger")
            (`PrimitiveComponent.SetMaterial` (`self.enemyModel_static`) 0 "/Game/Materials/MAT_Enemy_Main_Charger.MAT_Enemy_Main_Charger")
            (elif (`|EnumEquality` (`self.attackType`) "EAT_defense")
              (`PrimitiveComponent.SetMaterial` _enemymodel_weapon 0 "/Game/Materials/MAT_Enemy_Main_Defender.MAT_Enemy_Main_Defender")
              (`PrimitiveComponent.SetMaterial` (`self.enemyModel_static`) 0 "/Game/Materials/MAT_Enemy_Main_Defender.MAT_Enemy_Main_Defender")
              (elif (`|EnumEquality` (`self.attackType`) "EAT_mines")
                (`PrimitiveComponent.SetMaterial` _enemymodel_weapon 0 "/Game/Materials/MAT_Enemy_Main_Defender.MAT_Enemy_Main_Defender")))))))
    (:`then_11`
      ;[1 1 1] charger explode
      (if (`self.bDoExplode`)
        (`/Engine/EditorBlueprintResources/StandardMacros.DoOnce` false
          (:`Completed`
            (`GameplayStatics.PlaySoundAtLocation` "/Game/Sounds/cues/SND_chargerExplosion.SND_chargerExplosion" _returnvalue (struct) 1.0 1.0 0.0 null null null)
            (`|SpawnActorFromClass` "/Game/Objects/EnemyObjects/BP_ChargerExplosion.BP_ChargerExplosion_C" (`KismetMathLibrary.MakeTransform` _returnvalue) "AlwaysSpawn" "OverrideRootScale" null null)
            (set `self.healthValue` 0.0)))))
    (:`then_12`
      ;[1 1 1] set aggro range display size (12 == 400)
      (`/Engine/EditorBlueprintResources/StandardMacros.DoOnce` false
        (:`Completed`
          (`SceneComponent.SetWorldScale3D` (`self.AggroDisplaySphere`) (`KismetMathLibrary.MakeVector` _returnvalue_4 _returnvalue_4 _returnvalue_4)))))
    (:`then_13`
      ;[1 1 1] fill waypoints locations
      (`/Engine/EditorBlueprintResources/StandardMacros.DoOnce` false
        (:`Completed`
          (if (> (`KismetArrayLibrary.Array_Length` _patrolwaypoints) 0)
            (for _array_element _patrolwaypoints
              (`KismetArrayLibrary.Array_AddUnique` (`self.patrolWayPointLocations`) (`self.K2_GetActorLocation` _array_element)))))))))

(event `self.aggroRangeDisplay.OnComponentEndOverlap`
  (params (OverlappedComponent :type "PrimitiveComponent Object Reference") (OtherActor :type "Actor Object Reference") (OtherComp :type "PrimitiveComponent Object Reference") (OtherBodyIndex :type Integer))
  ;[1 1 1] collisions
  (`self.OnOverlapEnd` OverlappedComponent OtherActor OtherComp OtherBodyIndex))

(fn `UserConstructionScript`
  (`parent.UserConstructionScript`))