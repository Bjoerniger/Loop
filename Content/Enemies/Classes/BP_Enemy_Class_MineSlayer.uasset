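; MineSlayer enemy class, a child Blueprint that builds on parent enemy logic and sets its AttackType to Clean on BeginPlay.
; Each Tick adds a fixed roll step to the world rotation of the DefenderRings1 component, so its spin speed depends on frame rate.
; The same Tick hides the rings whenever IsAlive is false.
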(event `self.ReceiveBeginPlay`
  (`parent.ReceiveBeginPlay`)
  (set `self.attackType` "EAT_clean"))

(event `self.ReceiveTick`
  (params (DeltaSeconds :type "Float (single-precision)"))
  (bind _defenderrings1 (`self.DefenderRings1`))
  (bind (_returnvalue_roll _returnvalue_pitch _returnvalue_yaw) (`KismetMathLibrary.BreakRotator` (`SceneComponent.K2_GetComponentRotation` _defenderrings1)))
  (`parent.ReceiveTick` DeltaSeconds)
  (`|ExecutionSequence`
    (:`then_0`
      (`SceneComponent.K2_SetWorldRotation` _defenderrings1 (`KismetMathLibrary.MakeRotator` (+ _returnvalue_roll 5.0) _returnvalue_pitch _returnvalue_yaw) false false))
    (:`then_1`
      (if (not (`self.bIsAlive`))
        (`SceneComponent.SetVisibility` (`self.DefenderRings1`) false false)))))

(fn `UserConstructionScript`
  (`parent.UserConstructionScript`))