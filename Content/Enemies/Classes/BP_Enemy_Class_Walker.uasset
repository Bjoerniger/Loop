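; BP_Enemy_Class_Walker is the walker enemy, a child Blueprint that sets its attack type to Walker and extends the parent's BeginPlay and Tick.
; Each tick it can manually roll the chassis mesh from the inverted aim pitch, then, while alive, fires projectiles with sound from its muzzle whenever shooting is allowed.
; On death it disables collision on its three body components and hides its point light once.
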(event `self.ReceiveBeginPlay`
  (`parent.ReceiveBeginPlay`)
  (set `self.attackType` "EAT_walker"))

(event `self.ReceiveTick`
  (params (DeltaSeconds :type "Float (single-precision)"))
  (bind _enemy_ball_advanced_0wing (`self.Enemy_Ball_Advanced_0wing`))
  (bind (_walkerchasisrotation_roll _walkerchasisrotation_pitch) (`KismetMathLibrary.BreakRotator` (`self.walkerChasisRotation`)))
  (bind _attacktype (`self.attackType`))
  (bind _muzzlelocation_walker (`self.MuzzleLocation_Walker`))
  (bind (_returnvalue_roll _returnvalue_pitch _returnvalue_yaw) (`KismetMathLibrary.BreakRotator` (`SceneComponent.K2_GetComponentRotation` _enemy_ball_advanced_0wing)))
  (`parent.ReceiveTick` DeltaSeconds)
  (`|ExecutionSequence`
    (:`then_0`
      ;[1 1 1] manual chasis aim for walkers, janz dreckiger voodoo
      (if (`self.bAimWalkerChasis`)
        (`SceneComponent.K2_SetWorldRotation` _enemy_ball_advanced_0wing (`KismetMathLibrary.MakeRotator` (* _walkerchasisrotation_pitch -1.0) _returnvalue_pitch _returnvalue_yaw) false false)))
    (:`then_1`
      ;[1 1 1] shoot
      (if (`self.bIsAlive`)
        (if (`|EnumEquality` _attacktype "EAT_range")
          (if (`self.bCanShoot`) :!label _label
            (`|SpawnActorFromClass` (`self.BulletType`) (`KismetMathLibrary.MakeTransform` (`SceneComponent.K2_GetComponentLocation` _muzzlelocation_walker) (`SceneComponent.K2_GetComponentRotation` _muzzlelocation_walker)) "AlwaysSpawn" "OverrideRootScale" null null)
            (`GameplayStatics.PlaySoundAtLocation` (`self.ShotSound`) (`self.K2_GetActorLocation`) (struct) 0.02 1.1 0.0 null null null)
            (set `self.bCanShoot` false)
            (set `self.shotFrequencyValue` 0.0))
          (elif (`|EnumEquality` _attacktype "EAT_walker")
            (goto _label)))))
    (:`then_2`
      ;[1 1 1] death
      (if (not (`self.bIsAlive`))
        (`/Engine/EditorBlueprintResources/StandardMacros.DoOnce` false
          (:`Completed`
            (`PrimitiveComponent.SetCollisionEnabled` (`self.Enemy_Ball_Advanced_Spider`) "NoCollision")
            (`PrimitiveComponent.SetCollisionEnabled` (`self.Enemy_Ball_Advanced_0wing`) "NoCollision")
            (`PrimitiveComponent.SetCollisionEnabled` (`self.Enemy_Ball_Advanced_Weapon`) "NoCollision")
            (`SceneComponent.SetVisibility` (`self.PointLight`) false false)))))))

(fn `UserConstructionScript`
  (`parent.UserConstructionScript`))