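; Defender enemy class for a side-scroller, extending a parent enemy with a shield that spins while neutral and snaps toward the player otherwise.
; Player bullets drain shield health, reset its regen timer and alert the enemy; charged hits also destroy the Defender itself, not the bullet.
; Tick disables the shield and aim laser at zero health or death.
; It also projects the player's aim onto an LOS plane, moving an optionally visible marker.
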(event `self.ReceiveBeginPlay`
  (`parent.ReceiveBeginPlay`)
  (set `self.attackType` "EAT_defense")
  (set `self.shieldFront` (`SceneComponent.K2_GetComponentRotation` (`self.ShieldSpinner`))))

(event `self.ReceiveTick`
  (params (DeltaSeconds :type "Float (single-precision)"))
  (bind (_returnvalue_roll _returnvalue_pitch _returnvalue_yaw) (`KismetMathLibrary.BreakRotator` (`self.K2_GetActorRotation`)))
  (bind (_returnvalue_roll_2 _returnvalue_pitch_2) (`KismetMathLibrary.BreakRotator` (`self.K2_GetActorRotation`)))
  (bind _shieldspinner (`self.ShieldSpinner`))
  (bind _arrow1_0 (`self.Arrow1_0`))
  (bind _losplane (`self.LOSPlane`))
  (bind _losplane_2 (`self.LOSPlane`))
  (bind _returnvalue (`SceneComponent.K2_GetComponentToWorld` _losplane))
  (bind (_returnvalue_roll_3 _returnvalue_pitch_3 _returnvalue_yaw_2) (`KismetMathLibrary.BreakRotator` (`SceneComponent.K2_GetComponentRotation` _shieldspinner)))
  (bind _returnvalue_2 (+ _returnvalue_yaw_2 (`self.rotationSpeed`)))
  (`parent.ReceiveTick` DeltaSeconds)
  (`|ExecutionSequence`
    (:`then_0`
      ;[1 1 1] shield rotation
      (if (`|EnumEquality` (`self.aggroState`) "EAS_neutral")
        (if (> _returnvalue_2 -360.0)
          ;;[1 1 1 1 14] rotation
          (`SceneComponent.K2_SetWorldRotation` _shieldspinner (`KismetMathLibrary.MakeRotator` _returnvalue_roll_3 _returnvalue_pitch_3 _returnvalue_2) false false)
          (else
            (`SceneComponent.K2_SetWorldRotation` _shieldspinner (`KismetMathLibrary.MakeRotator` _returnvalue_roll_3 _returnvalue_pitch_3) false false)))
        (else
          (bind _returnvalue_3 (`self.GetDirectionToPlayer`))
          (if (== _returnvalue_3 2)
            ;;[1 1 1 1 14] fronts
            (`SceneComponent.K2_SetWorldRotation` _shieldspinner (`KismetMathLibrary.MakeRotator` _returnvalue_roll_2 _returnvalue_pitch_2 -90.0) false false)
            (elif (== _returnvalue_3 1)
              (`SceneComponent.K2_SetWorldRotation` _shieldspinner (`KismetMathLibrary.MakeRotator` _returnvalue_roll_2 _returnvalue_pitch_2 90.0) false false))))))
    (:`then_1`
      ;[1 1 1] disable shields on 0
      (if (> (`self.defenderShieldHealthValue`) 0.0)
        (if (not (`self.bIsAlive`))
          (`PrimitiveComponent.SetCollisionEnabled` (`self.ShieldCollision`) "NoCollision" :!label _label)
          (`SceneComponent.SetVisibility` (`self.ShieldWall`) false true)
          (`SceneComponent.SetVisibility` (`self.BP_EnemyAimLaser`) false true))
        (else
          (goto _label))))
    (:`then_2`
      (if true
        ;[1 1 1] LOS stuff
        (bind _asside_scroller_character (cast `/Game/SideScrollerCPP/Blueprints/SideScrollerCharacter` (`GameplayStatics.GetPlayerCharacter` 0)))
        (set `self.intersectionLOS` (`SceneComponent.K2_GetComponentLocation` _arrow1_0))
        (bind _arrowright (`/Game/SideScrollerCPP/Blueprints/SideScrollerCharacter.ArrowRight` _asside_scroller_character))
        (bind _returnvalue_4 (`SceneComponent.K2_GetComponentLocation` _arrowright))
        (bind (_t _intersection) (`KismetMathLibrary.LinePlaneIntersection_OriginNormal` _returnvalue_4 (+ (* (`KismetMathLibrary.GetForwardVector` (`SceneComponent.K2_GetComponentRotation` _arrowright)) 1000.0) _returnvalue_4) (`KismetMathLibrary.MakeVector` (.x (.location _returnvalue)) (.y (.location _returnvalue)) (.z (.location _returnvalue))) (`SceneComponent.GetUpVector` _losplane)))
        (`SceneComponent.K2_SetWorldLocation` _arrow1_0 (`KismetMathLibrary.MakeVector` (.x _intersection) (.y _intersection) (.z _intersection)) true false)))
    (:`then_3`
      ;[1 1 1] rotate LOS plane
      (if true
        (if (> _returnvalue_yaw 0.0)
          (`SceneComponent.K2_SetWorldRotation` _losplane_2 (`KismetMathLibrary.MakeRotator` 0.0 90.0 90.0) false false)
          (elif (< _returnvalue_yaw 0.0)
            (`SceneComponent.K2_SetWorldRotation` _losplane_2 (`KismetMathLibrary.MakeRotator` 0.0 90.0 -90.0) false false)))))
    (:`then_5`
      (`SceneComponent.SetHiddenInGame` (`self.Arrow1_0`) (not (`self.bShowLOSPos`)) false))))

(event `self.ShieldCollision.OnComponentBeginOverlap`
  (params (OverlappedComponent :type "PrimitiveComponent Object Reference") (OtherActor :type "Actor Object Reference") (OtherComp :type "PrimitiveComponent Object Reference") (OtherBodyIndex :type Integer) (bFromSweep :type Boolean) (SweepResult :type "HitResult Structure (by ref)"))
  (bind _returnvalue (`KismetSystemLibrary.GetDisplayName` OtherActor))
  (bind _defendershieldhealthvalue (`self.defenderShieldHealthValue`))
  ;[1 1 1] shield dmg
  ;;[1 1 1] normal bullet
  (if (`KismetStringLibrary.Contains` _returnvalue "PlayerBullet_Main")
    (if (> _defendershieldhealthvalue 0.0)
      (set `self.defenderShieldHealthValue` (- _defendershieldhealthvalue 1.0))
      (set `self.defenderShieldRegenTimerValue` 0.0)
      (set `self.bIsAllerted` true)
      (if (`KismetSystemLibrary.IsValid` OtherActor)
        (`self.K2_DestroyActor` OtherActor)))
    (else
      ;;[1 1 1] charged bullet
      (if (`KismetStringLibrary.Contains` _returnvalue "PlayerBullet_Charged")
        (if (> _defendershieldhealthvalue 0.0)
          (set `self.defenderShieldHealthValue` (- _defendershieldhealthvalue 5.0))
          (set `self.defenderShieldRegenTimerValue` 0.0)
          (set `self.bIsAllerted` true)
          (if (`KismetSystemLibrary.IsValid` OtherActor)
            (`self.K2_DestroyActor`)))))))

(fn `UserConstructionScript`
  (`parent.UserConstructionScript`))