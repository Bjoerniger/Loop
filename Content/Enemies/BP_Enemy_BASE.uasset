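; Base enemy for a side-scroller, handling health, hit reactions, ranged fire and death, with health and aggro widgets bound on BeginPlay.
; Tick polls externally set flags, applying bullet, crit or stomp damage by matching hitter names.
; Player dashes temporarily switch collision profiles on a timer.
; At zero health it disables triggers and swaps the static mesh for a physics-simulated destructible, while Ranged types spawn bullets whenever Shoot is set.
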(event `self.ReceiveBeginPlay`
  (`|ExecutionSequence`
    (:`then_0`
      ;[1 1 1] init vars for UI
      (bind _returnvalue (`|CreateWidget` "/Game/UI/UI_EnemyHealthBPBar.UI_EnemyHealthBPBar_C"))
      (set `self.Ref_HealthWidget` _returnvalue))
    (:`then_1`
      (bind _asui_enemy_health_bar (cast `/Game/UI/UI_EnemyHealthBar` (`WidgetComponent.GetUserWidgetObject` (`self.UI_Health`))))
      (set `/Game/UI/UI_EnemyHealthBar.Enemy` self _asui_enemy_health_bar))
    (:`then_2`
      (bind _returnvalue_2 (`|CreateWidget` "/Game/UI/UI_EnemyAggro.UI_EnemyAggro_C"))
      (set `self.Ref_AggroWidget` _returnvalue_2))
    (:`then_3`
      (bind _asui_enemy_aggro (cast `/Game/UI/UI_EnemyAggro` (`WidgetComponent.GetUserWidgetObject` (`self.UI_Aggro`))))
      (set `/Game/UI/UI_EnemyAggro.Enemy` self _asui_enemy_aggro))))

(event `self.ReceiveTick`
  (params (DeltaSeconds :type "Float (single-precision)"))
  (bind _core (`self.Core`))
  (bind _enemymodel_destructable (`self.EnemyModel_Destructable`))
  (bind _enemymodel_static (`self.EnemyModel_Static`))
  (bind _thehitcomp (`self.theHitComp`))
  (bind _enemymodel_static_2 (`self.EnemyModel_Static`))
  (bind _enemymodel_destructable_2 (`self.EnemyModel_Destructable`))
  (bind _arrow (`self.Arrow`))
  (bind _returnvalue (`KismetSystemLibrary.GetObjectName` (`self.theHitMan`)))
  (bind _returnvalue_2 (`KismetSystemLibrary.GetObjectName` (`self.theHitMan`)))
  (bind (_relativerotation_roll _relativerotation_pitch _relativerotation_yaw) (`KismetMathLibrary.BreakRotator` (`SceneComponent.RelativeRotation` _core)))
  (`|ExecutionSequence`
    (:`then_0`
      ;[1 1 1] vars
      ;;[1 1 1] set death on health 0
      (if (<= (`self.healthValue`) 0.0)
        (set `self.bIsAlive` false)))
    (:`then_1`
      ;;[1 1 1] set health %
      (set `self.healthReturnValue` (/ (`self.healthValue`) (`self.healthMax`))))
    (:`then_2`
      ;[1 1 1] dash
      (if (`self.bBeenDashed`)
        (if (`self.bIsAlive`)
          (if (< (`self.dashedTimerValue`) (`self.dashedTimerMax`))
            (set `self.dashedTimerValue` (+ DeltaSeconds (`self.dashedTimerValue`)))
            (else
              (set `self.bBeenDashed` false)
              (set `self.dashedTimerValue` 0.0)
              (`PrimitiveComponent.SetCollisionProfileName` (`self.BodyTriggerVolume`) "EnemyCollision"))))))
    (:`then_3`
      ;[1 1 1] on death
      (if (not (`self.bIsAlive`))
        (`/Engine/EditorBlueprintResources/StandardMacros.DoOnce` false
          (:`Completed`
            (`PrimitiveComponent.SetCollisionEnabled` (`self.bodyTriggerVolume`) "NoCollision")
            (`PrimitiveComponent.SetCollisionEnabled` (`self.headTriggerVolume`) "NoCollision")
            (`SceneComponent.SetVisibility` _enemymodel_static_2 false false)
            (`SceneComponent.SetHiddenInGame` _enemymodel_static_2 true false)
            (`PrimitiveComponent.SetCollisionProfileName` (`self.EnemyModel_Destructable`) "NoEnemyCollision")
            (`PrimitiveComponent.SetCollisionProfileName` (`self.EnemyModel_Static`) "NoEnemyCollision")
            (`PrimitiveComponent.SetCollisionProfileName` (`self.bodyTriggerVolume`) "NoEnemyCollision")
            (`PrimitiveComponent.SetCollisionProfileName` (`self.headTriggerVolume`) "NoEnemyCollision")
            (`SceneComponent.SetHiddenInGame` _enemymodel_destructable false false)
            (`PrimitiveComponent.SetEnableGravity` _enemymodel_destructable true)
            (`PrimitiveComponent.WakeRigidBody` _enemymodel_destructable "None")
            (`PrimitiveComponent.SetSimulatePhysics` _enemymodel_destructable true)
            (`PrimitiveComponent.SetCollisionEnabled` _enemymodel_destructable "QueryAndPhysics")))))
    (:`then_4`
      (set `self.bGotGrav` (`PrimitiveComponent.IsGravityEnabled` (`self.EnemyModel_Destructable`))))
    (:`then_5`
      ;[1 1 1] hit by player and death
      (if (`self.bBeenHit`)
        (if (`KismetStringLibrary.Contains` _returnvalue_2 "PlayerBullet")
          (set `self.healthValue` (- (`self.healthValue`) (`self.damageCast`)) :!label _label)
          (set `self.bBeenHit` false)
          (elif (`KismetStringLibrary.Contains` _returnvalue_2 "Stomper")
            (goto _label)
            (elif (`KismetSystemLibrary.IsValid` _thehitcomp)
              (if (`ActorComponent.ComponentHasTag` _thehitcomp "TriggerCheck")
                (bind _asside_scroller_character (cast `/Game/SideScrollerCPP/Blueprints/SideScrollerCharacter` (`GameplayStatics.GetPlayerCharacter` 0)))
                (set `self.bBeenDashed` true)
                (if (`self.bIsAlive`)
                  (if (`UnholyCharacter.isDashing` _asside_scroller_character)
                    (`PrimitiveComponent.SetCollisionProfileName` _enemymodel_static "NoEnemyCollision" :!label _label_2)
                    (`PrimitiveComponent.SetCollisionProfileName` (`self.BodyTriggerVolume`) "NoEnemyCollision")
                    (elif (<= (`self.healthValue`) 0.0)
                      (goto _label_2)
                      (else
                        (`PrimitiveComponent.SetCollisionProfileName` _enemymodel_static "EnemyCollision")
                        (`PrimitiveComponent.SetCollisionProfileName` (`self.BodyTriggerVolume`) "EnemyCollision"))))
                  (else
                    (goto _label_2)))))))))
    (:`then_6`
      ;[1 1 1] collision settings
      (if (`self.bGotGrav`)
        (if (`PrimitiveComponent.IsGravityEnabled` (`self.EnemyModel_Destructable`))
          (`PrimitiveComponent.SetCollisionEnabled` _enemymodel_destructable_2 "QueryAndPhysics")
          (`SceneComponent.SetVisibility` _enemymodel_destructable_2 true false)
          (`PrimitiveComponent.SetSimulatePhysics` (`self.Core`) true)
          (else
            (`PrimitiveComponent.SetCollisionEnabled` _enemymodel_destructable_2 "NoCollision")
            (`SceneComponent.SetVisibility` _enemymodel_destructable_2 false false)))))
    (:`then_7`
      ;[1 1 1] simple core rotation
      (if true
        (`SceneComponent.K2_AddLocalRotation` _core (`KismetMathLibrary.MakeRotator` (+ _relativerotation_roll -1.0) (+ _relativerotation_pitch 1.0) (+ _relativerotation_yaw 2.0)) false false)))
    (:`then_8`
      ;[1 1 1] shoot
      (if (`|EnumEquality` (`self.attackType`) "EAT_range")
        (if (`self.bShoot`)
          (`|SpawnActorFromClass` "/Game/Objects/BP_EnemyBullet_Main.BP_EnemyBullet_Main_C" (`KismetMathLibrary.MakeTransform` (`SceneComponent.K2_GetComponentLocation` _arrow) (`SceneComponent.K2_GetComponentRotation` _arrow)) "Undefined" "OverrideRootScale" null null)
          (set `self.bShoot` false)
          (set `self.shotFrequencyValue` 0.0))))
    (:`then_9`
      ;[1 1 1] crit by player and death
      (if (`self.bBeenCrit`)
        (if (`KismetStringLibrary.Contains` _returnvalue "PlayerBullet")
          (bind _asunholy_character (cast `UnholyCharacter` (`GameplayStatics.GetPlayerCharacter` 0)))
          (set `self.healthValue` (- (`self.healthValue`) (* (`self.damageCast`) (`UnholyCharacter.critMultiplier` _asunholy_character))))
          (set `self.bBeenCrit` false)
          (elif (`KismetStringLibrary.Contains` _returnvalue "Stomper")
            (set `self.healthValue` (- (`self.healthValue`) (`self.damageCast`)))
            (set `self.bBeenCrit` false)))))))

(fn `UserConstructionScript`)