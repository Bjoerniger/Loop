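; Trigger volume that switches the game to the level named in LevelName when the player or a TriggerCheck-tagged component overlaps its Box.
; On overlap it copies the UnholyCharacter's skills, health and jump count into GI_Loop, plays SoundToPlay and waits out its duration.
; Tick then sees LevelLoadingDone, sets GI_Loop's load flags and opens the level.
; Without a sound assigned, the overlap does nothing.
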(event `self.ReceiveTick`
  (params (DeltaSeconds :type "Float (single-precision)"))
  (if (`self.levelLoadingDone`)
    (bind _asgi_loop (cast `/Game/Level/GI_Loop` (`GameplayStatics.GetGameInstance`)))
    (set `/Game/Level/GI_Loop.S1_IsSavedGame` false _asgi_loop)
    (set `/Game/Level/GI_Loop.L_IsLevelLoad` true _asgi_loop)
    (`GameplayStatics.OpenLevel` (`KismetStringLibrary.Conv_StringToName` (`self.LevelName`)))))

(event `self.Box.OnComponentBeginOverlap`
  (params (OverlappedComponent :type "PrimitiveComponent Object Reference") (OtherActor :type "Actor Object Reference") (OtherComp :type "PrimitiveComponent Object Reference") (OtherBodyIndex :type Integer) (bFromSweep :type Boolean) (SweepResult :type "HitResult Structure (by ref)"))
  (bind _soundtoplay (`self.SoundToPlay`))
  (if (or (`ActorComponent.ComponentHasTag` OtherComp "TriggerCheck") (`self.ActorHasTag` OtherActor "Player"))
    (if (!= (`self.SoundToPlay`) null)
      (`|ExecutionSequence`
        (:`then_0`
          (bind _asunholy_character (cast `UnholyCharacter` (`GameplayStatics.GetPlayerCharacter` 0)))
          (bind _asgi_loop (cast `/Game/Level/GI_Loop` (`GameplayStatics.GetGameInstance`)))
          ;[1 1 1] add all vars that have to be saved
          (set `/Game/Level/GI_Loop.L_CanDash` (`UnholyCharacter.skills_CanDash` _asunholy_character) _asgi_loop)
          (set `/Game/Level/GI_Loop.L_CanWallJump` (`UnholyCharacter.skills_CanWallJump` _asunholy_character) _asgi_loop)
          (set `/Game/Level/GI_Loop.L_HealthMax` (`UnholyCharacter.healthMax` _asunholy_character) _asgi_loop)
          (set `/Game/Level/GI_Loop.L_HealthValue` (`UnholyCharacter.healthValue` _asunholy_character) _asgi_loop)
          (set `/Game/Level/GI_Loop.L_JumpCounter` (`UnholyCharacter.jumpCounterMax` _asunholy_character) _asgi_loop))
        (:`then_1`
          (`GameplayStatics.PlaySound2D` _soundtoplay 0.05 1.0 0.0 null null)
          (`KismetSystemLibrary.Delay` (`SoundBase.Duration` _soundtoplay))
          (set `self.levelLoadingDone` true))))))

(fn `UserConstructionScript`)