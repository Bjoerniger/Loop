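; BP_KillingField is a kill volume that restarts the current level when the player enters its box.
; Non-player actors that overlap it are destroyed.
; A DoOnce gates the player's death: in levels with "Mario" in the name, it zeroes UnholyCharacter health, disables movement and plays a sound, reloading after that sound's duration.
; Other levels reload immediately.
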(event `self.Box.OnComponentBeginOverlap`
  (params (OverlappedComponent :type "PrimitiveComponent Object Reference") (OtherActor :type "Actor Object Reference") (OtherComp :type "PrimitiveComponent Object Reference") (OtherBodyIndex :type Integer) (bFromSweep :type Boolean) (SweepResult :type "HitResult Structure (by ref)"))
  (bind _soundtoplay (`self.SoundToPlay`))
  (if (`self.ActorHasTag` OtherActor "Player")
    (`/Engine/EditorBlueprintResources/StandardMacros.DoOnce` false
      (:`Completed`
        (bind _returnvalue (`GameplayStatics.GetCurrentLevelName` true))
        (if (`KismetStringLibrary.Contains` _returnvalue "Mario")
          (bind _asunholy_character (cast `UnholyCharacter` (`GameplayStatics.GetPlayerCharacter` 0)))
          (set `UnholyCharacter.healthValue` 0.0 _asunholy_character)
          (set `UnholyCharacter.bAllowMovement` false _asunholy_character)
          (`GameplayStatics.PlaySound2D` _soundtoplay 1.0 1.0 0.0 null null)
          (`KismetSystemLibrary.Delay` (`SoundBase.Duration` _soundtoplay)))
        (`GameplayStatics.OpenLevel` (`KismetStringLibrary.Conv_StringToName` _returnvalue))))
    (else
      (`self.K2_DestroyActor` OtherActor))))

(fn `UserConstructionScript`)