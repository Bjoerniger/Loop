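; BP_artifact_main is an animated artifact object built from rings, strings and a cube component that spin continuously.
; Tick adds fixed local rotations to each component on differing axes and rates, without delta-time scaling, so spin speed follows frame rate.
; Leftover logic for a sphere pulsing between growing and shrinking around a maximum scale is disconnected and never runs.
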(event `self.ReceiveBeginPlay`)

(event `self.ReceiveTick`
  (params (DeltaSeconds :type "Float (single-precision)"))
  (`|ExecutionSequence`
    (:`then_0`
      (`SceneComponent.K2_AddLocalRotation` (`self.ring`) (`KismetMathLibrary.MakeRotator` 0.7 0.25) false false)
      (`SceneComponent.K2_AddLocalRotation` (`self.ring1`) (`KismetMathLibrary.MakeRotator` 0.4 0.0 0.125) false false)
      (`SceneComponent.K2_AddLocalRotation` (`self.ring2`) (`KismetMathLibrary.MakeRotator` 0.3 -0.3 0.25) false false)
      (`SceneComponent.K2_AddLocalRotation` (`self.artifact_string`) (`KismetMathLibrary.MakeRotator` 0.0 0.5 -0.5) false false)
      (`SceneComponent.K2_AddLocalRotation` (`self.artifact_string1`) (`KismetMathLibrary.MakeRotator` 0.0 1.0) false false))
    (:`then_1`
      (`SceneComponent.K2_AddLocalRotation` (`self.artifact_cubes`) (`KismetMathLibrary.MakeRotator` 0.05 -0.05 0.05) false false))))

(fn `UserConstructionScript`)