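; Health station actor that gradually restores the player's health while they stand inside its Box trigger.
; Box overlap begin and end events from actors tagged Player switch the DoHeal flag on and off.
; While the flag is set, Tick casts player character 0 to UnholyCharacter and adds a small fixed amount to HealthValue while it is below HealthMax.
; The increment ignores delta time, so healing speed depends on frame rate.
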(event `self.ReceiveTick`
  (params (DeltaSeconds :type "Float (single-precision)"))
  (if (`self.DoHeal`)
    (bind _asunholy_character (cast `UnholyCharacter` (`GameplayStatics.GetPlayerCharacter` 0)))
    (bind _healthvalue (`UnholyCharacter.healthValue` _asunholy_character))
    (if (< _healthvalue (`UnholyCharacter.healthMax` _asunholy_character))
      (set `UnholyCharacter.healthValue` (+ _healthvalue 0.1) _asunholy_character))))

(event `self.Box.OnComponentBeginOverlap`
  (params (OverlappedComponent :type "PrimitiveComponent Object Reference") (OtherActor :type "Actor Object Reference") (OtherComp :type "PrimitiveComponent Object Reference") (OtherBodyIndex :type Integer) (bFromSweep :type Boolean) (SweepResult :type "HitResult Structure (by ref)"))
  (if (`self.ActorHasTag` OtherActor "Player")
    (set `self.DoHeal` true)))

(event `self.Box.OnComponentEndOverlap`
  (params (OverlappedComponent :type "PrimitiveComponent Object Reference") (OtherActor :type "Actor Object Reference") (OtherComp :type "PrimitiveComponent Object Reference") (OtherBodyIndex :type Integer))
  (if (`self.ActorHasTag` OtherActor "Player")
    (set `self.DoHeal` false)))

(fn `UserConstructionScript`)