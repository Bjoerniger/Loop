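; Black hole actor whose outer sphere pulses in size, with no other behavior active.
; Each Tick adds or subtracts Growth from the sphere's world scale, flipping direction at the min and max limits, checked on X only.
; The step ignores delta time, so pulse speed follows frame rate.
; BeginPlay caches the starting scale without using it here, and a root-shrinking node is left unconnected.
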(event `self.ReceiveBeginPlay`
  (set `self.OuterSphereActualScale` (`SceneComponent.K2_GetComponentScale` (`self.Outer Sphere`))))

(event `self.ReceiveTick`
  (params (DeltaSeconds :type "Float (single-precision)"))
  (bind _outer_sphere (`self.Outer Sphere`))
  (bind _outer_sphere_2 (`self.Outer Sphere`))
  (bind _outerspheremaxscale_x (`KismetMathLibrary.BreakVector` (`self.OuterSphereMaxScale`)))
  (bind _outersphereminscale_x (`KismetMathLibrary.BreakVector` (`self.OuterSphereMinScale`)))
  (bind (_returnvalue_x _returnvalue_y _returnvalue_z) (`KismetMathLibrary.BreakVector` (`SceneComponent.K2_GetComponentScale` _outer_sphere_2)))
  (bind (_returnvalue_x_2 _returnvalue_y_2 _returnvalue_z_2) (`KismetMathLibrary.BreakVector` (`SceneComponent.K2_GetComponentScale` _outer_sphere)))
  (`|ExecutionSequence`
    (:`then_1`
      ;[1 1 1] pulse
      (if (`self.OutSphereGrowthDirection`)
        (if (<= _returnvalue_x _outerspheremaxscale_x)
          (`SceneComponent.SetWorldScale3D` _outer_sphere_2 (+ (`KismetMathLibrary.MakeVector` _returnvalue_x _returnvalue_y _returnvalue_z) (`self.growth`)))
          (else
            (set `self.OutSphereGrowthDirection` false)))
        (elif (> _returnvalue_x_2 _outersphereminscale_x)
          (`SceneComponent.SetWorldScale3D` _outer_sphere (- (`KismetMathLibrary.MakeVector` _returnvalue_x_2 _returnvalue_y_2 _returnvalue_z_2) (`self.growth`)))
          (else
            (set `self.OutSphereGrowthDirection` true)))))))

(fn `UserConstructionScript`)