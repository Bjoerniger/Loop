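; Charged player bullet actor that expires after BulletFlightTime and damages enemies it overlaps.
; Collider overlaps ignore the player pawn and match enemies by "Enemy" in the object name, writing BulletDamage into the Enemy's DamageCast variable.
; It then spawns a blue explosion and destroys itself, unless the overlapped component's name contains "Destructable", which lets it pass through.
; The graph runs no movement logic.
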(event `self.ReceiveBeginPlay`
  (`self.SetLifeSpan` (`self.bulletFlightTime`)))

(event `self.ReceiveTick`
  (params (DeltaSeconds :type "Float (single-precision)")))

(event `self.PlayerBulletCollider.OnComponentHit`
  (params (HitComponent :type "PrimitiveComponent Object Reference") (OtherActor :type "Actor Object Reference") (OtherComp :type "PrimitiveComponent Object Reference") (NormalImpulse :type "Vector Structure") (Hit :type "HitResult Structure (by ref)")))

(event `self.PlayerBulletCollider.OnComponentBeginOverlap`
  (params (OverlappedComponent :type "PrimitiveComponent Object Reference") (OtherActor :type "Actor Object Reference") (OtherComp :type "PrimitiveComponent Object Reference") (OtherBodyIndex :type Integer) (bFromSweep :type Boolean) (SweepResult :type "HitResult Structure (by ref)"))
  (bind _returnvalue_location (`KismetMathLibrary.BreakTransform` (`SceneComponent.K2_GetComponentToWorld` (`self.Cylinder`))))
  (if (!= OtherActor (`GameplayStatics.GetPlayerPawn` 0))
    (if (`KismetStringLibrary.Contains` (`KismetSystemLibrary.GetObjectName` OtherActor) "Enemy")
      (bind _asenemy (cast `Enemy` OtherActor))
      (set `Enemy.damageCast` (`self.bulletDamage`) _asenemy))
    (if (not (`KismetStringLibrary.Contains` (`KismetSystemLibrary.GetObjectName` OtherComp) "Destructable"))
      (`GameplayStatics.SpawnEmitterAtLocation` "/Game/StarterContent/Particles/P_Explosion_Blue.P_Explosion_Blue" _returnvalue_location (struct) (1.3 1.3 1.3) true "AutoRelease")
      (`self.K2_DestroyActor`))))

(fn `UserConstructionScript`)