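; BP_knockBackSphere is the player's expanding stomp knockback sphere, which records the enemies it reaches.
; It starts small with a maximum size extended by the character's stomp timer, then grows each tick while KnockBackUsed is set.
; Overlaps with enemy head trigger volumes add those actors to the character's KnockBackHitActors array; the damage logic is unconnected.
; At full size it waits, clears KnockBackUsed and destroys itself.
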(event `self.ReceiveBeginPlay`
  ;[1 1 1] set base vars
  (`SceneComponent.SetWorldScale3D` (`self.CollisionSphere`) (0.2 0.2 0.2))
  (`SceneComponent.SetWorldScale3D` (`self.Sphere`) (0.2 0.2 0.2))
  (bind _asunholy_character (cast `UnholyCharacter` (`GameplayStatics.GetPlayerCharacter` 0)))
  (set `self.maxSize` (+ (`self.maxSize`) (`UnholyCharacter.stompTimerValue` _asunholy_character))))

(event `self.ReceiveTick`
  (params (DeltaSeconds :type "Float (single-precision)"))
  (bind _maxsize_x (`KismetMathLibrary.BreakVector` (`self.maxSize`)))
  (bind _collisionsphere (`self.CollisionSphere`))
  (bind _returnvalue_x (`KismetMathLibrary.BreakVector` (`SceneComponent.K2_GetComponentScale` _collisionsphere)))
  ;[1 1 1] size growth & destroy
  (bind _asunholy_character (cast `UnholyCharacter` (`GameplayStatics.GetPlayerCharacter` 0)))
  (if (`UnholyCharacter.bKnockBackUsed` _asunholy_character)
    (if (< _returnvalue_x _maxsize_x)
      (`SceneComponent.SetWorldScale3D` (`self.Sphere`) (+ (`SceneComponent.K2_GetComponentScale` _collisionsphere) (`self.growth`)))
      (`SceneComponent.SetWorldScale3D` _collisionsphere (+ (`SceneComponent.K2_GetComponentScale` _collisionsphere) (`self.growth`)))
      (else
        (`KismetSystemLibrary.Delay` (`self.exploder duration`))
        (set `UnholyCharacter.bKnockBackUsed` false _asunholy_character)
        (`self.K2_DestroyActor`)))))

(event `self.CollisionSphere.OnComponentBeginOverlap`
  (params (OverlappedComponent :type "PrimitiveComponent Object Reference") (OtherActor :type "Actor Object Reference") (OtherComp :type "PrimitiveComponent Object Reference") (OtherBodyIndex :type Integer) (bFromSweep :type Boolean) (SweepResult :type "HitResult Structure (by ref)"))
  ;[1 1 1] deal dmg after stomp
)

(event `self.Sphere.OnComponentBeginOverlap`
  (params (OverlappedComponent :type "PrimitiveComponent Object Reference") (OtherActor :type "Actor Object Reference") (OtherComp :type "PrimitiveComponent Object Reference") (OtherBodyIndex :type Integer) (bFromSweep :type Boolean) (SweepResult :type "HitResult Structure (by ref)"))
  ;[1 1 1] add enemies to hit array
  (bind _asunholy_character (cast `UnholyCharacter` (`GameplayStatics.GetPlayerCharacter` 0)))
  (if (`KismetArrayLibrary.Array_Contains` (`UnholyCharacter.knockBackHitActors` _asunholy_character) OtherActor)
    _
    (elif (`self.ActorHasTag` OtherActor "Enemy")
      (if (`KismetStringLibrary.Contains` (`KismetSystemLibrary.GetDisplayName` OtherComp) "headTriggerVolume")
        (`KismetArrayLibrary.Array_AddUnique` (`UnholyCharacter.knockBackHitActors` _asunholy_character) OtherActor)))))

(fn `UserConstructionScript`)