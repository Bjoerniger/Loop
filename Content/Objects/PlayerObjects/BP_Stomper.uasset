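; BP_Stomper is the expanding damage sphere for the player's stomp attack.
; On BeginPlay it starts small and sets its maximum size from the player's base stomp size plus StompTimerValue.
; Tick grows the visual and collision spheres to that limit, then destroys the actor after a delay.
; Overlapped "Enemy"-tagged actors are flagged as hit, receiving damage scaled by StompTimerValue and the player as attacker.
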(event `self.ReceiveBeginPlay`
  (bind _returnvalue (`GameplayStatics.GetPlayerCharacter` 0))
  ;[1 1 1] set base vars
  (`SceneComponent.SetWorldScale3D` (`self.CollisionSphere`) (0.2 0.2 0.2))
  (`SceneComponent.SetWorldScale3D` (`self.Sphere`) (0.2 0.2 0.2))
  (bind _asside_scroller_character (cast `/Game/SideScrollerCPP/Blueprints/SideScrollerCharacter` _returnvalue))
  (bind _asunholy_character (cast `UnholyCharacter` _returnvalue))
  (set `self.maxSize` (+ (`/Game/SideScrollerCPP/Blueprints/SideScrollerCharacter.StomperMaxSize` _asside_scroller_character) (`UnholyCharacter.stompTimerValue` _asunholy_character))))

(event `self.ReceiveTick`
  (params (DeltaSeconds :type "Float (single-precision)"))
  (bind _maxsize_x (`KismetMathLibrary.BreakVector` (`self.maxSize`)))
  (bind _collisionsphere (`self.CollisionSphere`))
  (bind _returnvalue_x (`KismetMathLibrary.BreakVector` (`SceneComponent.K2_GetComponentScale` _collisionsphere)))
  ;[1 1 1] size growth & destroy
  (if (< _returnvalue_x _maxsize_x)
    (`SceneComponent.SetWorldScale3D` (`self.Sphere`) (+ (`SceneComponent.K2_GetComponentScale` _collisionsphere) (`self.growth`)))
    (`SceneComponent.SetWorldScale3D` _collisionsphere (+ (`SceneComponent.K2_GetComponentScale` _collisionsphere) (`self.growth`)))
    (else
      (`KismetSystemLibrary.Delay` (`self.exploder duration`))
      (`self.K2_DestroyActor`))))

(event `self.CollisionSphere.OnComponentBeginOverlap`
  (params (OverlappedComponent :type "PrimitiveComponent Object Reference") (OtherActor :type "Actor Object Reference") (OtherComp :type "PrimitiveComponent Object Reference") (OtherBodyIndex :type Integer) (bFromSweep :type Boolean) (SweepResult :type "HitResult Structure (by ref)"))
  ;[1 1 1] deal dmg after stomp
  (if (`self.ActorHasTag` OtherActor "Enemy")
    (bind _asenemy (cast `Enemy` OtherActor))
    (bind _asunholy_character (cast `UnholyCharacter` (`GameplayStatics.GetPlayerCharacter` 0)))
    (set `Enemy.bBeenHit` true _asenemy)
    (set `Enemy.damageCast` (* (`self.damage`) (`UnholyCharacter.stompTimerValue` _asunholy_character)) _asenemy)
    (set `Enemy.theHitMan` _asunholy_character _asenemy)))

(fn `UserConstructionScript`)