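; BP_muzzleFlash is a short-lived muzzle flash actor built from Plane and PlaneInner components.
; BeginPlay gives each plane its own random roll so flashes vary.
; Tick grows Plane's world scale by a fixed step per frame until it passes MaxGrowth, then shrinks it below zero and destroys the actor, with GrowthDirection tracking the phase.
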(event `self.ReceiveBeginPlay`
  (bind _plane (`self.Plane`))
  (bind _planeinner (`self.PlaneInner`))
  (bind (_relativerotation_roll _relativerotation_pitch _relativerotation_yaw) (`KismetMathLibrary.BreakRotator` (`SceneComponent.RelativeRotation` _planeinner)))
  (bind (_relativerotation_roll_2 _relativerotation_pitch_2 _relativerotation_yaw_2) (`KismetMathLibrary.BreakRotator` (`SceneComponent.RelativeRotation` _plane)))
  (`SceneComponent.K2_SetRelativeRotation` _plane (`KismetMathLibrary.MakeRotator` (`KismetMathLibrary.Conv_IntToDouble` (`KismetMathLibrary.RandomInteger` 90)) _relativerotation_pitch_2 _relativerotation_yaw_2) false false)
  (`SceneComponent.K2_SetRelativeRotation` _planeinner (`KismetMathLibrary.MakeRotator` (`KismetMathLibrary.Conv_IntToDouble` (`KismetMathLibrary.RandomInteger` 90)) _relativerotation_pitch _relativerotation_yaw) false false))

(event `self.ReceiveTick`
  (params (DeltaSeconds :type "Float (single-precision)"))
  (bind _plane (`self.Plane`))
  (bind _growth (`self.growth`))
  (bind _plane_2 (`self.Plane`))
  (bind _growth_2 (`self.growth`))
  (bind (_returnvalue_x _returnvalue_y _returnvalue_z) (`KismetMathLibrary.BreakVector` (`SceneComponent.K2_GetComponentScale` _plane)))
  (bind (_returnvalue_x_2 _returnvalue_y_2 _returnvalue_z_2) (`KismetMathLibrary.BreakVector` (`SceneComponent.K2_GetComponentScale` _plane_2)))
  (if (`self.growthDirection`)
    (if (<= _returnvalue_x_2 (`self.maxGrowth`))
      (`SceneComponent.SetWorldScale3D` _plane_2 (`KismetMathLibrary.MakeVector` (+ _returnvalue_x_2 _growth_2) (+ _returnvalue_y_2 _growth_2) (+ _returnvalue_z_2 _growth_2)))
      (else
        (set `self.growthDirection` false)))
    (elif (>= _returnvalue_x 0.0)
      (`SceneComponent.SetWorldScale3D` _plane (`KismetMathLibrary.MakeVector` (- _returnvalue_x _growth) (- _returnvalue_y _growth) (- _returnvalue_z _growth)))
      (else
        (`self.K2_DestroyActor`)))))

(fn `UserConstructionScript`)