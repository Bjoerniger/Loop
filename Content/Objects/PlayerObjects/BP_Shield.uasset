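; BP_Shield is a player shield actor that shows a spinning hex-material sphere which pulses when the shield is activated.
; BeginPlay creates a dynamic material instance on ShieldSphere.
; Tick writes the Opacity parameter and yaws the sphere in fixed per-frame steps, without delta time.
; While the UnholyCharacter player's ShieldActive is set, opacity ramps up then down at FadeInSpeed, then the actor clears that flag.
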(event `self.ReceiveBeginPlay`
  (bind _returnvalue (`PrimitiveComponent.CreateDynamicMaterialInstance` (`self.ShieldSphere`) 0 "/Game/Materials/MAT_I_Shield_Hex.MAT_I_Shield_Hex" "None"))
  (`MaterialInstanceDynamic.SetScalarParameterValue` _returnvalue "Opacity" 1.0))

(event `self.ReceiveTick`
  (params (DeltaSeconds :type "Float (single-precision)"))
  (bind _shieldopacityvalue (`self.ShieldOpacityValue`))
  (`|ExecutionSequence`
    (:`then_0`
      (`MaterialInstanceDynamic.SetScalarParameterValue` (stale `self.ReceiveBeginPlay` _returnvalue) "Opacity" (`self.ShieldOpacityValue`)))
    (:`then_1`
      ;[1 1 1] fader value
      (bind _asunholy_character (cast `UnholyCharacter` (`GameplayStatics.GetPlayerCharacter` 0)))
      (if true
        (if (`UnholyCharacter.bShieldActive` _asunholy_character)
          (if (`self.FadeIn`)
            (if (< _shieldopacityvalue 2.0)
              (set `self.ShieldOpacityValue` (+ _shieldopacityvalue (`self.FadeInSpeed`)))
              (else
                (set `self.FadeIn` false)))
            (elif (> _shieldopacityvalue 0.0)
              (set `self.ShieldOpacityValue` (- _shieldopacityvalue (`self.FadeInSpeed`)))
              (else
                (set `self.FadeIn` true)
                (set `UnholyCharacter.bShieldActive` false _asunholy_character)))))))
    (:`then_2`
      (`SceneComponent.K2_AddLocalRotation` (`self.ShieldSphere`) (`KismetMathLibrary.MakeRotator` 0.0 0.0 10.0) false false))))

(fn `UserConstructionScript`)