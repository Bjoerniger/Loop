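; A level switch that lets the player permanently activate a linked BP_EnergyDoor.
; Trigger overlaps set the in-range flags and pass the target object's name to UnholyCharacter, clearing them shortly after exit.
; Tick polls the character's use flag, activates ObjectToActivate if its name contains "Door", then keeps the plate on its active material.
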(event `self.ReceiveBeginPlay`)

(event `self.ReceiveTick`
  (params (DeltaSeconds :type "Float (single-precision)"))
  (bind _objecttoactivate (`self.ObjectToActivate`))
  (`|ExecutionSequence`
    (:`then_1`
      ;[1 1 1] Activated by Player
      (bind _asunholy_character (cast `UnholyCharacter` (`GameplayStatics.GetPlayerCharacter` 0)))
      (if (`self.PlayerInRange_D`)
        (if (`UnholyCharacter.bUsableInRange` _asunholy_character)
          (if (`UnholyCharacter.bUsableActivated` _asunholy_character)
            (if (`KismetStringLibrary.Contains` (`KismetSystemLibrary.GetObjectName` _objecttoactivate) "Door" true)
              (bind _asbp_energy_door (cast `/Game/Objects/LevelBlocks/BP_EnergyDoor` _objecttoactivate))
              (set `/Game/Objects/LevelBlocks/BP_EnergyDoor.IsActivated` true _asbp_energy_door)
              (set `self.WasActivated` true)
              (set `UnholyCharacter.bUsableInRange` false _asunholy_character))))))
    (:`then_2`
      (if (`self.WasActivated`)
        (`PrimitiveComponent.SetMaterial` (`self.Plate`) 0 "/Game/Materials/MAT_Active.MAT_Active")))))

(event `self.TriggerArea.OnComponentBeginOverlap`
  (params (OverlappedComponent :type "PrimitiveComponent Object Reference") (OtherActor :type "Actor Object Reference") (OtherComp :type "PrimitiveComponent Object Reference") (OtherBodyIndex :type Integer) (bFromSweep :type Boolean) (SweepResult :type "HitResult Structure (by ref)"))
  ;[1 1 1] activate + plate position
  (if (`self.ActorHasTag` OtherActor "Player")
    (bind _asunholy_character (cast `UnholyCharacter` (`GameplayStatics.GetPlayerCharacter` 0)))
    (if (not (`self.WasActivated`))
      (set `UnholyCharacter.bUsableInRange` true _asunholy_character)
      (set `UnholyCharacter.ActivateObjectName` (`KismetSystemLibrary.GetObjectName` (`self.ObjectToActivate`)) _asunholy_character)
      (set `self.PlayerInRange_D` true))))

(event `self.TriggerArea.OnComponentEndOverlap`
  (params (OverlappedComponent :type "PrimitiveComponent Object Reference") (OtherActor :type "Actor Object Reference") (OtherComp :type "PrimitiveComponent Object Reference") (OtherBodyIndex :type Integer))
  ;[1 1 1] activate + plate position
  (if (`ActorComponent.ComponentHasTag` OtherComp "TriggerCheck")
    (`KismetSystemLibrary.Delay` 0.1)
    (bind _asunholy_character (cast `UnholyCharacter` (`GameplayStatics.GetPlayerCharacter` 0)))
    (set `UnholyCharacter.bUsableInRange` false _asunholy_character)
    (set `UnholyCharacter.ActivateObjectName` "" _asunholy_character)
    (set `self.PlayerInRange_D` false)))

(fn `UserConstructionScript`)