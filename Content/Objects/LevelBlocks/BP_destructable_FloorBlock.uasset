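; A destructible floor block that dissolves and vanishes after an actor with "Stomper" in its display name overlaps its collision box.
; The overlap sets a Destruct flag, which Tick polls to create a dynamic dissolve material on the cube and play a timeline driving its dissolve amount.
; Tick also disables the cube's collision partway through the dissolve and destroys the actor once it completes.
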(event `self.ReceiveTick`
  (params (DeltaSeconds :type "Float (single-precision)"))
  (bind _cube (`self.Cube`))
  (`|ExecutionSequence`
    (:`then_0`
      (if (`self.destruct`)
        (bind _returnvalue (`PrimitiveComponent.CreateDynamicMaterialInstance` _cube 0 "/Game/Materials/MAT_I_dissolve.MAT_I_dissolve" "None"))
        (bind (_direction _newtrack_0) (`Timeline|Timeline_0`)
          (:`Update`
            (bind _output_get (set `self.destructAmmount` _newtrack_0))
            (`MaterialInstanceDynamic.SetScalarParameterValue` _returnvalue "DissolveAmmount" _output_get)))))
    (:`then_1`
      (if (>= (`self.destructAmmount`) 0.6)
        (`PrimitiveComponent.SetCollisionEnabled` _cube "NoCollision")))
    (:`then_2`
      (if (>= (`self.destructAmmount`) 1.0)
        (`self.K2_DestroyActor`)))))

(event `self.CollisionBox.OnComponentBeginOverlap`
  (params (OverlappedComponent :type "PrimitiveComponent Object Reference") (OtherActor :type "Actor Object Reference") (OtherComp :type "PrimitiveComponent Object Reference") (OtherBodyIndex :type Integer) (bFromSweep :type Boolean) (SweepResult :type "HitResult Structure (by ref)"))
  ;[1 1 1] 1: floorblock
  (if (`KismetStringLibrary.Contains` (`KismetSystemLibrary.GetDisplayName` OtherActor) "Stomper")
    (set `self.destruct` true)))

(fn `UserConstructionScript`)