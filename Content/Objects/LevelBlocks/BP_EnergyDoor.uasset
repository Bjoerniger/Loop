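; BP_EnergyDoor is a level-block door whose energy shield rises to open when IsActivated is true.
; Tick polls that flag, plays the open sound through a never-reset DoOnce, and raises the shield a fixed, frame-rate-dependent step toward EnergyShieldMaxLoc.
; While rising, it disables shield collision and applies the active material to four meshes.
; When inactive, it restores collision and the inactive material but never lowers the shield.
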(event `self.ReceiveTick`
  (params (DeltaSeconds :type "Float (single-precision)"))
  (bind _energyshield (`self.EnergyShield`))
  (bind _staticmesh (`self.StaticMesh`))
  (bind (_returnvalue_x _returnvalue_y _returnvalue_z) (`KismetMathLibrary.BreakVector` (`SceneComponent.K2_GetComponentLocation` _energyshield)))
  (bind (_returnvalue_x_2 _returnvalue_y_2 _returnvalue_z_2) (`KismetMathLibrary.BreakVector` (`SceneComponent.K2_GetComponentLocation` (`self.EnergyShieldMaxLoc`))))
  (if (`self.IsActivated`)
    (`|ExecutionSequence`
      (:`then_0`
        (`/Engine/EditorBlueprintResources/StandardMacros.DoOnce` false
          (:`Completed`
            (`GameplayStatics.PlaySoundAtLocation` "/Game/Sounds/cues/SND_Door_open.SND_Door_open" (`SceneComponent.K2_GetComponentLocation` (`self.DefaultSceneRoot`)) (struct) 0.15 1.0 0.0 null null null))))
      (:`then_1`
        (if (< _returnvalue_z _returnvalue_z_2)
          (`SceneComponent.K2_SetWorldLocation` _energyshield (`KismetMathLibrary.MakeVector` _returnvalue_x _returnvalue_y (+ _returnvalue_z 1.0)) false false)
          (`PrimitiveComponent.SetMaterial` _staticmesh 0 "/Game/Materials/MAT_Active_solid.MAT_Active_solid")
          (`PrimitiveComponent.SetMaterial` (`self.StaticMesh3`) 0 "/Game/Materials/MAT_Active_solid.MAT_Active_solid")
          (`PrimitiveComponent.SetMaterial` (`self.StaticMesh2`) 0 "/Game/Materials/MAT_Active_solid.MAT_Active_solid")
          (`PrimitiveComponent.SetMaterial` (`self.StaticMesh1`) 0 "/Game/Materials/MAT_Active_solid.MAT_Active_solid")
          (`PrimitiveComponent.SetCollisionEnabled` _energyshield "NoCollision"))))
    (else
      (`PrimitiveComponent.SetCollisionEnabled` _energyshield "QueryAndPhysics")
      (`PrimitiveComponent.SetMaterial` _staticmesh 0 "/Game/Materials/MAT_InActive.MAT_InActive")
      (`PrimitiveComponent.SetMaterial` (`self.StaticMesh3`) 0 "/Game/Materials/MAT_InActive.MAT_InActive")
      (`PrimitiveComponent.SetMaterial` (`self.StaticMesh2`) 0 "/Game/Materials/MAT_InActive.MAT_InActive")
      (`PrimitiveComponent.SetMaterial` (`self.StaticMesh1`) 0 "/Game/Materials/MAT_InActive.MAT_InActive"))))

(fn `UserConstructionScript`)