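; Level block that activates a linked energy door once the enemies in its box are dead.
; On BeginPlay it records every Enemy overlapping the box in an alive list and total count.
; Each Tick it polls all Enemy actors, removing dead ones still overlapping the box from the list.
; While the list is empty, including when none start inside, it sets IsActivated on the BP_EnergyDoor.
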(event `self.ReceiveBeginPlay`
  (bind _outactors (`GameplayStatics.GetAllActorsOfClass` "/Script/Unholy.Enemy"))
  (for _array_element _outactors
    (if (`PrimitiveComponent.IsOverlappingActor` (`self.Box`) _array_element)
      (set `self.EnemiesTotal` (+ (`self.EnemiesTotal`) 1))
      (`KismetArrayLibrary.Array_AddUnique` (`self.EnemiesAlive`) _array_element))))

(event `self.ReceiveTick`
  (params (DeltaSeconds :type "Float (single-precision)"))
  (bind _dooractortoactivate (`self.DoorActorToActivate`))
  (`|ExecutionSequence`
    (:`then_0`
      (bind _outactors (`GameplayStatics.GetAllActorsOfClass` "/Script/Unholy.Enemy"))
      (for _array_element _outactors
        (if (`PrimitiveComponent.IsOverlappingActor` (`self.Box`) _array_element)
          (bind _asenemy (cast `Enemy` _array_element))
          (`/Engine/EditorBlueprintResources/StandardMacros.IsValid` _asenemy
            (:`Is Valid`
              (if (not (`Enemy.bIsAlive` _asenemy))
                (`KismetArrayLibrary.Array_RemoveItem` (`self.EnemiesAlive`) _asenemy)))))))
    (:`then_1`
      (if (== (`KismetArrayLibrary.Array_Length` (`self.EnemiesAlive`)) 0)
        (`/Engine/EditorBlueprintResources/StandardMacros.IsValid` _dooractortoactivate
          (:`Is Valid`
            (bind _asbp_energy_door (cast `/Game/Objects/LevelBlocks/BP_EnergyDoor` _dooractortoactivate))
            (set `/Game/Objects/LevelBlocks/BP_EnergyDoor.IsActivated` true _asbp_energy_door)))))))

(fn `UserConstructionScript`)