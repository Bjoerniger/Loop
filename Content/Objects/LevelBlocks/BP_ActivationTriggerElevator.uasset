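; Pressure plate that activates a linked Elevator when a Player-tagged actor steps on it, sinking by StepDepth.
; One second after the player leaves, the plate rises and re-arms through chained DoOnce gates, also deactivating the elevator if Switch is set.
; With Switch, Tick also deactivates it when TriggerTime is non-positive, otherwise counting a timer that is never compared.
; BeginPlay also enables the UnholyCharacter's movement.
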(event `self.ReceiveBeginPlay`
  (set `self.plateStartLocation` (`SceneComponent.K2_GetComponentLocation` (`self.Plate`)))
  (bind _asunholy_character (cast `UnholyCharacter` (`GameplayStatics.GetPlayerPawn` 0)))
  (set `UnholyCharacter.bAllowMovement` true _asunholy_character))

(event `self.ReceiveTick`
  (params (DeltaSeconds :type "Float (single-precision)"))
  ;[1 1 1] deactivate if triggered switch timer
  (if (`self.Switch`)
    (bind _aselevator (cast `Elevator` (`self.ObjectToActivate`)))
    (if (`Elevator.bIsActivated` _aselevator)
      (if (>= 0.0 (`self.TriggerTime`))
        (set `Elevator.bIsActivated` false _aselevator)
        (else
          (set `self.TriggerActiveTimer` (+ (`self.TriggerActiveTimer`) DeltaSeconds)))))))

(event `self.TriggerArea.OnComponentBeginOverlap`
  (params (OverlappedComponent :type "PrimitiveComponent Object Reference") (OtherActor :type "Actor Object Reference") (OtherComp :type "PrimitiveComponent Object Reference") (OtherBodyIndex :type Integer) (bFromSweep :type Boolean) (SweepResult :type "HitResult Structure (by ref)"))
  (bind (_platestartlocation_x _platestartlocation_y _platestartlocation_z) (`KismetMathLibrary.BreakVector` (`self.plateStartLocation`)))
  ;[1 1 1] activate + plate position
  (if (`self.ActorHasTag` OtherActor "Player")
    (`/Engine/EditorBlueprintResources/StandardMacros.DoOnce` false :!label _label
      (:`Completed`
        (bind _aselevator (cast `Elevator` (`self.ObjectToActivate`)))
        (set `Elevator.bIsActivated` true _aselevator)
        (`SceneComponent.K2_SetWorldLocation` (`self.Plate`) (`KismetMathLibrary.MakeVector` _platestartlocation_x _platestartlocation_y (- _platestartlocation_z (`self.stepDepth`))) false false)
        (`|ExecutionSequence`
          (:`then_0`
            (goto _label_3 :!via `Reset`))
          (:`then_1`
            (goto _label_2 :!via `Reset`)))))))

(event `self.TriggerArea.OnComponentEndOverlap`
  (params (OverlappedComponent :type "PrimitiveComponent Object Reference") (OtherActor :type "Actor Object Reference") (OtherComp :type "PrimitiveComponent Object Reference") (OtherBodyIndex :type Integer))
  ;[1 1 1] activate + plate position
  (if (`self.ActorHasTag` OtherActor "Player")
    (`KismetSystemLibrary.Delay` 1.0)
    (`/Engine/EditorBlueprintResources/StandardMacros.DoOnce` false :!label _label_2
      (:`Completed`
        (`SceneComponent.K2_SetWorldLocation` (`self.Plate`) (`self.plateStartLocation`) false false)
        (if (`self.Switch`)
          (`/Engine/EditorBlueprintResources/StandardMacros.DoOnce` false :!label _label_3
            (:`Completed`
              (bind _aselevator (cast `Elevator` (`self.ObjectToActivate`)))
              (set `Elevator.bIsActivated` false _aselevator)
              (goto _label :!via `Reset`)))
          (else
            (goto _label :!via `Reset`)))))))

(fn `UserConstructionScript`)