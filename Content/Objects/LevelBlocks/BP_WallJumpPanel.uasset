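; Wall-jump panel level block that lets the player's UnholyCharacter wall jump off it, with its cube shown only while the character has the wall-jump skill.
; A box overlap with a "TriggerCheck"-tagged component flags the player as at the panel.
; While flagged, Tick enables CanWallJump when airborne and derives JumpDirection from the arrow's negated forward Y component.
; Leaving the box clears the flag and CanWallJump.
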(event `self.ReceiveTick`
  (params (DeltaSeconds :type "Float (single-precision)"))
  (bind _cube (`self.Cube`))
  (`|ExecutionSequence`
    (:`then_0`
      (bind _asunholy_character (cast `UnholyCharacter` (`GameplayStatics.GetPlayerCharacter` 0)))
      (if (`UnholyCharacter.skills_CanWallJump` _asunholy_character)
        (`SceneComponent.SetVisibility` _cube true false)
        (else
          (`SceneComponent.SetVisibility` _cube false false))))
    (:`then_1`
      (if (`self.charAtWalljump`)
        (bind _asunholy_character_2 (cast `UnholyCharacter` (`GameplayStatics.GetPlayerCharacter` 0)))
        (if (not (`UnholyCharacter.bIsOnGround` _asunholy_character_2))
          (set `UnholyCharacter.bCanWallJump` true _asunholy_character_2))))
    (:`then_2`
      ;[1 1 1] set wallhug direction
      (if (`self.charAtWalljump`)
        (bind _asunholy_character_3 (cast `UnholyCharacter` (`GameplayStatics.GetPlayerCharacter` 0)))
        (set `UnholyCharacter.jumpDirection` (* (`KismetMathLibrary.Conv_RotatorToVector` (`SceneComponent.K2_GetComponentRotation` (`self.Arrow`))) (0.0 -1.0 0.0)) _asunholy_character_3)))))

(event `self.Box.OnComponentBeginOverlap`
  (params (OverlappedComponent :type "PrimitiveComponent Object Reference") (OtherActor :type "Actor Object Reference") (OtherComp :type "PrimitiveComponent Object Reference") (OtherBodyIndex :type Integer) (bFromSweep :type Boolean) (SweepResult :type "HitResult Structure (by ref)"))
  (if (`ActorComponent.ComponentHasTag` OtherComp "TriggerCheck")
    (set `self.charAtWalljump` true)))

(event `self.Box.OnComponentEndOverlap`
  (params (OverlappedComponent :type "PrimitiveComponent Object Reference") (OtherActor :type "Actor Object Reference") (OtherComp :type "PrimitiveComponent Object Reference") (OtherBodyIndex :type Integer))
  (if (`ActorComponent.ComponentHasTag` OtherComp "TriggerCheck")
    (set `self.charAtWalljump` false)
    (bind _asunholy_character (cast `UnholyCharacter` (`GameplayStatics.GetPlayerCharacter` 0)))
    (set `UnholyCharacter.bCanWallJump` false _asunholy_character)))

(fn `UserConstructionScript`)