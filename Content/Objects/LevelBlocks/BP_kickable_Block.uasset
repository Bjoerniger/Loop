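; Level block that the player can knock away with a knockback sphere and that stops charged player bullets.
; Its Box overlap destroys charged bullets, matched by display name, with a blue explosion, or flags knockback for actors tagged KnockbackSphere.
; When flagged, Tick enables physics on the Cube and applies a force away from the player along Y plus upward lift, slightly weaker on the +Y side, then clears the flag.
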(event `self.ReceiveTick`
  (params (DeltaSeconds :type "Float (single-precision)"))
  (bind _returnvalue (`GameplayStatics.GetPlayerCharacter` 0))
  (bind _knockback_force (`self.knockback force`))
  (bind _knockback_force_2 (`self.knockback force`))
  (bind _cube (`self.Cube`))
  (bind (_returnvalue_x _returnvalue_y) (`KismetMathLibrary.BreakVector` (`self.K2_GetActorLocation` self)))
  (bind (_returnvalue_x_2 _returnvalue_y_2) (`KismetMathLibrary.BreakVector` (`SceneComponent.K2_GetComponentLocation` (`Actor.RootComponent` _returnvalue))))
  (bind (_returnvalue_x_3 _returnvalue_y_3) (`KismetMathLibrary.BreakVector` (- (`KismetMathLibrary.MakeVector` 0.0 _returnvalue_y) (`KismetMathLibrary.MakeVector` 0.0 _returnvalue_y_2))))
  (if (`self.isKnockedBack`)
    (`PrimitiveComponent.SetSimulatePhysics` (`self.Cube`) true)
    (cast `UnholyCharacter` _returnvalue)
    ;[1 1 1] right
    (if (< _returnvalue_y_3 0.0)
      (`PrimitiveComponent.AddForce` _cube (`KismetMathLibrary.MakeVector` 0.0 (* _knockback_force_2 -1.0) (/ _knockback_force_2 1.0)) "None" true)
      (set `self.isKnockedBack` false :!label _label)
      (else
        ;[1 1 1] letf
        (if (> _returnvalue_y_3 0.0)
          (`PrimitiveComponent.AddForce` _cube (`KismetMathLibrary.MakeVector` 0.0 (* _knockback_force 1.0) (/ _knockback_force 1.5)) "None" true)
          (goto _label))))))

(event `self.Box.OnComponentBeginOverlap`
  (params (OverlappedComponent :type "PrimitiveComponent Object Reference") (OtherActor :type "Actor Object Reference") (OtherComp :type "PrimitiveComponent Object Reference") (OtherBodyIndex :type Integer) (bFromSweep :type Boolean) (SweepResult :type "HitResult Structure (by ref)"))
  (if (`KismetStringLibrary.Contains` (`KismetSystemLibrary.GetDisplayName` OtherActor) "PlayerBullet_Charged")
    (`GameplayStatics.SpawnEmitterAtLocation` "/Game/StarterContent/Particles/P_Explosion_Blue.P_Explosion_Blue" (`self.K2_GetActorLocation` OtherActor) (struct) (0.5 0.5 0.5) true "AutoRelease")
    (`self.K2_DestroyActor` OtherActor)
    (elif (`KismetSystemLibrary.IsValid` OtherActor)
      (if (`self.ActorHasTag` OtherActor "KnockbackSphere")
        (set `self.isKnockedBack` true)))))

(fn `UserConstructionScript`)