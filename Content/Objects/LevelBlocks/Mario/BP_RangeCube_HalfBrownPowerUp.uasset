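; Mario-style level block that releases a power-up once when the player hits it while jumping.
; Box overlap accepts an UnholyCharacter with a TriggerCheck component tag or Player actor tag, then reads IsJumping from player character 0.
; A DoOnce gate, never reset here, spawns the PowerUpToSpawn class at the PUSpawnLocation transform.
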(event `self.Box.OnComponentBeginOverlap`
  (params (OverlappedComponent :type "PrimitiveComponent Object Reference") (OtherActor :type "Actor Object Reference") (OtherComp :type "PrimitiveComponent Object Reference") (OtherBodyIndex :type Integer) (bFromSweep :type Boolean) (SweepResult :type "HitResult Structure (by ref)"))
  (cast `UnholyCharacter` OtherActor)
  (if (or (`ActorComponent.ComponentHasTag` OtherComp "TriggerCheck") (`self.ActorHasTag` OtherActor "Player"))
    (bind _asunholy_character (cast `UnholyCharacter` (`GameplayStatics.GetPlayerCharacter` 0)))
    (if (`UnholyCharacter.bIsJumping` _asunholy_character)
      (`/Engine/EditorBlueprintResources/StandardMacros.DoOnce` false
        (:`Completed`
          (`|SpawnActorFromClass` (`self.PowerUpToSpawn`) (`SceneComponent.K2_GetComponentToWorld` (`self.PU_SpawnLocation`)) "Undefined" "OverrideRootScale" null null))))))

(fn `UserConstructionScript`)