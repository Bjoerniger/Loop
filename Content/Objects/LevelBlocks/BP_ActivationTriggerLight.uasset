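; BP_ActivationTriggerLight is a level block trigger that switches on a linked BP_flickeringSpotLight.
; When an actor tagged Player overlaps TriggerArea, a DoOnce lets it cast ObjectToActivate and set IsActive to true a single time.
; Tick also sets IsActive to true every frame while Switch is set.
; Despite a comment about timed deactivation, nothing here turns the light off.
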(event `self.ReceiveBeginPlay`)

(event `self.ReceiveTick`
  (params (DeltaSeconds :type "Float (single-precision)"))
  ;[1 1 1] deactivate if triggered switch timer
  (if (`self.Switch`)
    (bind _asbp_flickering_spot_light (cast `/Game/Objects/lights/BP_flickeringSpotLight` (`self.ObjectToActivate`)))
    (if true
      (set `/Game/Objects/lights/BP_flickeringSpotLight.isActive` true _asbp_flickering_spot_light))))

(event `self.TriggerArea.OnComponentBeginOverlap`
  (params (OverlappedComponent :type "PrimitiveComponent Object Reference") (OtherActor :type "Actor Object Reference") (OtherComp :type "PrimitiveComponent Object Reference") (OtherBodyIndex :type Integer) (bFromSweep :type Boolean) (SweepResult :type "HitResult Structure (by ref)"))
  ;[1 1 1] activate + plate position
  (if (`self.ActorHasTag` OtherActor "Player")
    (`/Engine/EditorBlueprintResources/StandardMacros.DoOnce` false
      (:`Completed`
        (bind _asbp_flickering_spot_light (cast `/Game/Objects/lights/BP_flickeringSpotLight` (`self.ObjectToActivate`)))
        (set `/Game/Objects/lights/BP_flickeringSpotLight.isActive` true _asbp_flickering_spot_light)))))

(fn `UserConstructionScript`)