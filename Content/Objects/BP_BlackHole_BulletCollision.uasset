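; BP_BlackHole_BulletCollision is a short-lived black hole actor, apparently an effect for bullet collisions, that shrinks and removes itself.
; Each Tick, while OutSphereGrowthDirection is false, it subtracts Growth from the OuterSphere's world scale, then destroys the actor once X reaches the minimum.
; The step is per frame, without delta-time scaling.
; BeginPlay stores the starting scale; only the shrink half of the pulse is wired, and overlap handling is disabled.
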(event `self.ReceiveBeginPlay`
  (set `self.OuterSphereActualScale` (`SceneComponent.K2_GetComponentScale` (`self.Outer Sphere`))))

(event `self.ReceiveTick`
  (params (DeltaSeconds :type "Float (single-precision)"))
  (bind _outer_sphere (`self.Outer Sphere`))
  (bind _outersphereminscale_x (`KismetMathLibrary.BreakVector` (`self.OuterSphereMinScale`)))
  (bind (_returnvalue_x _returnvalue_y _returnvalue_z) (`KismetMathLibrary.BreakVector` (`SceneComponent.K2_GetComponentScale` _outer_sphere)))
  (`|ExecutionSequence`
    (:`then_1`
      ;[1 1 1] pulse
      (if (`self.OutSphereGrowthDirection`)
        _
        (elif (> _returnvalue_x _outersphereminscale_x)
          (`SceneComponent.SetWorldScale3D` _outer_sphere (- (`KismetMathLibrary.MakeVector` _returnvalue_x _returnvalue_y _returnvalue_z) (`self.growth`)))
          (else
            (`self.K2_DestroyActor`)))))))

(fn `UserConstructionScript`)