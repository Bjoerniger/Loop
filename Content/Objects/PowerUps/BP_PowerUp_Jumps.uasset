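; A jump power-up pickup that raises the player's maximum jump count by one.
; Its IconBox spins in yaw every tick as a visual cue.
; Overlapping the trigger box with a TriggerCheck-tagged component or Player-tagged actor fires once, printing a debug message, incrementing JumpCounterMax on the player's UnholyCharacter, then destroying the pickup.
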(event `self.ReceiveBeginPlay`)

(event `self.ReceiveTick`
  (params (DeltaSeconds :type "Float (single-precision)"))
  (bind _iconbox (`self.IconBox`))
  (bind (_returnvalue_roll _returnvalue_pitch _returnvalue_yaw) (`KismetMathLibrary.BreakRotator` (`SceneComponent.K2_GetComponentRotation` _iconbox)))
  (`|ExecutionSequence`
    (:`then_0`
      ;[1 1 1] spin
      (`SceneComponent.K2_SetWorldRotation` _iconbox (`KismetMathLibrary.MakeRotator` _returnvalue_roll _returnvalue_pitch (+ _returnvalue_yaw 1.0)) false false))))

(event `self.Box.OnComponentBeginOverlap`
  (params (OverlappedComponent :type "PrimitiveComponent Object Reference") (OtherActor :type "Actor Object Reference") (OtherComp :type "PrimitiveComponent Object Reference") (OtherBodyIndex :type Integer) (bFromSweep :type Boolean) (SweepResult :type "HitResult Structure (by ref)"))
  ;[1 1 1] trigger
  (if (or (`ActorComponent.ComponentHasTag` OtherComp "TriggerCheck") (`self.ActorHasTag` OtherActor "Player"))
    (`/Engine/EditorBlueprintResources/StandardMacros.DoOnce` false
      (:`Completed`
        (`KismetSystemLibrary.PrintString` "jump cnt max ++!")
        (bind _asunholy_character (cast `UnholyCharacter` (`GameplayStatics.GetPlayerCharacter` 0)))
        (set `UnholyCharacter.jumpCounterMax` (+ (`UnholyCharacter.jumpCounterMax` _asunholy_character) 1) _asunholy_character)
        (`self.K2_DestroyActor`)))))

(fn `UserConstructionScript`)