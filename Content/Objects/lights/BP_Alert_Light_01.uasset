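; BP_Alert_Light_01 is a light prop that pulses red-emissive when its Alert flag is set and shows blue when not.
; Tick sets the Cube material and RectLight colour every frame, using LightColourAlert during alert and black otherwise.
; During alert, LightDirection ping-pongs the intensity between BaseIntensity and MaxIntensity in FlashRate steps per tick, so flash speed depends on frame rate.
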(event `self.ReceiveTick`
  (params (DeltaSeconds :type "Float (single-precision)"))
  (bind _rectlight (`self.RectLight`))
  (bind _cube (`self.Cube`))
  (bind _intensity (`LightComponentBase.Intensity` _rectlight))
  (bind _intensity_2 (`LightComponentBase.Intensity` _rectlight))
  (if (`self.Alert`)
    (`PrimitiveComponent.SetMaterial` _cube 0 "/Game/Materials/lights/MAT_I_Emissive_Red.MAT_I_Emissive_Red")
    (`LightComponent.SetLightColor` _rectlight (`self.Light Colour Alert`) true)
    (if (`self.lightDirection`)
      (if (< _intensity_2 (`self.max Intensity`))
        (`LightComponent.SetIntensity` _rectlight (+ _intensity_2 (`self.FlashRate`)))
        (else
          (set `self.lightDirection` false)))
      (elif (> _intensity (`self.base Intensity`))
        (`LightComponent.SetIntensity` _rectlight (- _intensity (`self.FlashRate`)))
        (else
          (set `self.lightDirection` true))))
    (else
      (`PrimitiveComponent.SetMaterial` _cube 0 "/Game/Materials/lights/MAT_I_Emissive_Blue.MAT_I_Emissive_Blue")
      (`LightComponent.SetLightColor` :`self` _rectlight))))

(fn `UserConstructionScript`)