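; BP_FloatingLight_01_blue is a floating light actor, blue by its name, that jitters around in the level.
; Each Tick moves its Sphere component by a random relative offset on all three axes, bounded by plus or minus MovementRange.
; The offsets accumulate as an unclamped, frame-rate-dependent random walk.
; BeginPlay stores the starting location in CenterPos, but the movement never uses it to pull the sphere back.
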(event `self.ReceiveBeginPlay`
  (set `self.CenterPos` (`SceneComponent.K2_GetComponentLocation` (`self.Sphere`))))

(event `self.ReceiveTick`
  (params (DeltaSeconds :type "Float (single-precision)"))
  (bind _movementrange (`self.movementRange`))
  (bind _returnvalue (* _movementrange -1.0))
  (`SceneComponent.K2_AddRelativeLocation` (`self.Sphere`) (`KismetMathLibrary.MakeVector` (`KismetMathLibrary.RandomFloatInRange` _movementrange _returnvalue) (`KismetMathLibrary.RandomFloatInRange` _movementrange _returnvalue) (`KismetMathLibrary.RandomFloatInRange` _movementrange _returnvalue)) false false))

(fn `UserConstructionScript`)