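; BP_EnemyAimLaser is an enemy aim-laser actor that shows the aggro state of its parent BP_Enemy_Ball through the beam's color.
; Every Tick it casts its parent actor and sets the outer cylinder's material to orange for Allert or red for Neutral, leaving other states unchanged.
; When the parent enemy is no longer alive, it hides itself in game.
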(event `self.ReceiveTick`
  (params (DeltaSeconds :type "Float (single-precision)"))
  (bind _lazercylinder_outer (`self.lazerCylinder_outer`))
  (bind _returnvalue (`KismetSystemLibrary.IsValid` _lazercylinder_outer))
  (bind _asbp_enemy_ball (cast `/Game/Enemies/Base/BP_Enemy_Ball` (`self.GetParentActor`)))
  (if (`Enemy.bIsAlive` _asbp_enemy_ball)
    (bind _aggrostate (`Enemy.aggroState` _asbp_enemy_ball))
    (if (`|EnumEquality` _aggrostate "EAS_allert")
      (if _returnvalue
        (`PrimitiveComponent.SetMaterial` _lazercylinder_outer 0 "/Game/Materials/MAT_lazer_orange.MAT_lazer_orange"))
      (elif (`|EnumEquality` _aggrostate "EAS_neutral")
        (if _returnvalue
          (`PrimitiveComponent.SetMaterial` _lazercylinder_outer 0 "/Game/Materials/MAT_lazer_red.MAT_lazer_red"))))
    (else
      (`self.SetActorHiddenInGame` true))))

(fn `UserConstructionScript`)