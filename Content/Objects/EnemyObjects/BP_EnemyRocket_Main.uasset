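; Homing rocket projectile that, despite its EnemyRocket name, damages Enemy-tagged actors and ignores the player.
; The homingMissile event sets the projectile's homing target to the given target's mesh, and BeginPlay limits lifespan to the flight time.
; Any non-player overlap explodes and destroys it once, first subtracting BulletDamage directly from an enemy's HealthValue.
; Disconnected leftover logic for player damage and bullet penetration never runs.
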(event `self.EnemyBulletCollider.OnComponentBeginOverlap`
  (params (OverlappedComponent :type "PrimitiveComponent Object Reference") (OtherActor :type "Actor Object Reference") (OtherComp :type "PrimitiveComponent Object Reference") (OtherBodyIndex :type Integer) (bFromSweep :type Boolean) (SweepResult :type "HitResult Structure (by ref)"))
  (bind _returnvalue (`self.K2_GetActorLocation`))
  (bind _returnvalue_2 (`self.K2_GetActorLocation`))
  (if (`self.ActorHasTag` OtherActor "Player")
    _
    (elif (`self.ActorHasTag` OtherActor "Enemy")
      ;[1 1 1] damatsch
      (`/Engine/EditorBlueprintResources/StandardMacros.DoOnce` false
        (:`Completed`
          (`GameplayStatics.SpawnEmitterAtLocation` "/Game/StarterContent/Particles/P_Explosion_Blue.P_Explosion_Blue" _returnvalue (struct) (4.0 4.0 4.0))
          (bind _asenemy (cast `Enemy` OtherActor))
          ;;[1 1 1] deal dmg
          (set `Enemy.healthValue` (- (`Enemy.healthValue` _asenemy) (`self.bulletDamage`)) _asenemy)
          (`GameplayStatics.PlaySoundAtLocation` "/Game/Sounds/cues/SND_RocketExplosion.SND_RocketExplosion" _returnvalue (struct) 1.0 1.0 0.0 null null null)
          (`self.K2_DestroyActor`)))
      (else
        ;[1 1 1] explosion
        (`/Engine/EditorBlueprintResources/StandardMacros.DoOnce` false
          (:`Completed`
            (`GameplayStatics.SpawnEmitterAtLocation` "/Game/StarterContent/Particles/P_Explosion_Blue.P_Explosion_Blue" _returnvalue_2 (struct) (4.0 4.0 4.0))
            (`GameplayStatics.PlaySoundAtLocation` "/Game/Sounds/cues/SND_RocketExplosion.SND_RocketExplosion" _returnvalue_2 (struct) 1.0 1.0 0.0 null null null)
            (`self.K2_DestroyActor`)))))))

(event `self.ReceiveBeginPlay`
  (`self.SetLifeSpan` (`self.bulletFlightTime`)))

(event `homingMissile`
  (params (aimTarget :type "Enemy Object Reference"))
  ;[1 1 1] set homing missile
  (set `ProjectileMovementComponent.HomingTargetComponent` (`Character.Mesh` aimTarget) (`self.ProjectileMovement`)))

(event `self.ReceiveTick`
  (params (DeltaSeconds :type "Float (single-precision)")))

(fn `UserConstructionScript`)