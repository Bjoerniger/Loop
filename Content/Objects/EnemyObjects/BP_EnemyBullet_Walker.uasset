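; Walker enemy bullet that damages the player on overlap, spawns a small explosion and destroys itself, or expires after its flight time.
; Overlapping a player bullet, detected by display name, also destroys it.
; A player bullet with penetration above one loses a point and continues; otherwise it is destroyed too and a BP_BlackHole_BulletCollision spawns.
; The logic setting projectile movement speed from Speed is disconnected.
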(event `self.ReceiveBeginPlay`
  (`self.SetLifeSpan` (`self.bulletFlightTime`)))

(event `self.ReceiveTick`
  (params (DeltaSeconds :type "Float (single-precision)")))

(event `self.EnemyBulletCollider.OnComponentBeginOverlap`
  (params (OverlappedComponent :type "PrimitiveComponent Object Reference") (OtherActor :type "Actor Object Reference") (OtherComp :type "PrimitiveComponent Object Reference") (OtherBodyIndex :type Integer) (bFromSweep :type Boolean) (SweepResult :type "HitResult Structure (by ref)"))
  (bind _returnvalue_location (`KismetMathLibrary.BreakTransform` (`SceneComponent.K2_GetComponentToWorld` (`self.Sphere`))))
  ;[1 1 1] if player has been hit
  (if (`self.ActorHasTag` OtherActor "Player")
    (bind _asunholy_character (cast `UnholyCharacter` OtherActor))
    (`UnholyCharacter.DealDamage` _asunholy_character (`self.bulletDamage`))
    (`GameplayStatics.SpawnEmitterAtLocation` "/Game/StarterContent/Particles/P_Explosion.P_Explosion" _returnvalue_location (struct) (0.3 0.3 0.3) true "AutoRelease")
    (`self.K2_DestroyActor` :!label _label)
    (else
      ;[1 1 1] if player bullet, check for penetration and mb destroy
      (if (`KismetSystemLibrary.IsValid` OtherActor)
        (if (`KismetStringLibrary.Contains` (`KismetSystemLibrary.GetDisplayName` OtherActor) "PlayerBullet")
          (bind _asbp_player_bullet_main (cast `/Game/Objects/PlayerObjects/BP_PlayerBullet_Main` OtherActor))
          (bind _penetration (`/Game/Objects/PlayerObjects/BP_PlayerBullet_Main.penetration` _asbp_player_bullet_main))
          (if (> _penetration 1.0)
            (set `/Game/Objects/PlayerObjects/BP_PlayerBullet_Main.penetration` (- _penetration 1.0) _asbp_player_bullet_main)
            (goto _label)
            (else
              (`self.K2_DestroyActor` OtherActor)
              (`|SpawnActorFromClass` "/Game/Objects/BP_BlackHole_BulletCollision.BP_BlackHole_BulletCollision_C" (`KismetMathLibrary.MakeTransform` (`self.K2_GetActorLocation`) (struct) (0.8 0.8 0.8)) "Undefined" "OverrideRootScale" null null)
              (goto _label))))))))

(fn `UserConstructionScript`)